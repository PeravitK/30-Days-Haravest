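; Mole AI character for an animal event that targets crops and flees from the player, driven by blackboard keys and AnimBP_Mole.
; RunCollision overlaps set IsRunAway while BP_Char is inside, and any begin overlap stops the digging animation.
; ResetFromTargetDestroyed destroys all TargetSign actors, stops digging and movement, pulses TargetCropDestroyed and clears HaveTarget.
; Its State component is hidden on BeginPlay.
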(event `self.ReceiveBeginPlay`
  (`SceneComponent.SetVisibility` (`self.State`) false false))

(event `self.ReceiveTick`
  (params (DeltaSeconds :type "Float (single-precision)")))

(event `self.RunCollision.OnComponentBeginOverlap`
  (params (OverlappedComponent :type "PrimitiveComponent Object Reference") (OtherActor :type "Actor Object Reference") (OtherComp :type "PrimitiveComponent Object Reference") (OtherBodyIndex :type Integer) (bFromSweep :type Boolean) (SweepResult :type "HitResult Structure (by ref)"))
  (bind _asanim_bp_mole (cast `/Game/30DH/Event/AnimalEvent/AnimBP_Mole` (`SkeletalMeshComponent.GetAnimInstance` (`self.Mesh`))))
  (set `/Game/30DH/Event/AnimalEvent/AnimBP_Mole.isDigging` false _asanim_bp_mole)
  (cast `/Game/30DH/Character/BP_Char` OtherActor)
  (`BlackboardComponent.SetValueAsBool` (`AIBlueprintHelperLibrary.GetBlackboard` (`AIBlueprintHelperLibrary.GetAIController` self)) "IsRunAway" true))

(event `self.RunCollision.OnComponentEndOverlap`
  (params (OverlappedComponent :type "PrimitiveComponent Object Reference") (OtherActor :type "Actor Object Reference") (OtherComp :type "PrimitiveComponent Object Reference") (OtherBodyIndex :type Integer))
  (bind _returnvalue (`AIBlueprintHelperLibrary.GetBlackboard` (`AIBlueprintHelperLibrary.GetAIController` self)))
  (cast `/Game/30DH/Character/BP_Char` OtherActor)
  (`/Engine/EditorBlueprintResources/StandardMacros.IsValid` self
    (:`Is Valid`
      (`/Engine/EditorBlueprintResources/StandardMacros.IsValid` _returnvalue
        (:`Is Valid`
          (`BlackboardComponent.SetValueAsBool` _returnvalue "IsRunAway" false))))))

(fn `ResetFromTargetDestroyed`
  (bind _returnvalue (`AIBlueprintHelperLibrary.GetAIController` self))
  (bind _returnvalue_2 (`AIBlueprintHelperLibrary.GetBlackboard` _returnvalue))
  (bind _outactors (`GameplayStatics.GetAllActorsOfClass` "/Game/30DH/Event/AnimalEvent/TargetSign.TargetSign_C"))
  (for _array_element _outactors
    (`self.K2_DestroyActor` _array_element))
  (bind _asanim_bp_mole (cast `/Game/30DH/Event/AnimalEvent/AnimBP_Mole` (`SkeletalMeshComponent.GetAnimInstance` (`self.Mesh`))))
  (set `/Game/30DH/Event/AnimalEvent/AnimBP_Mole.isDigging` false _asanim_bp_mole)
  (`Controller.StopMovement` _returnvalue)
  (`BlackboardComponent.SetValueAsBool` _returnvalue_2 "TargetCropDestroyed" true)
  (`BlackboardComponent.SetValueAsBool` _returnvalue_2 "TargetCropDestroyed" false)
  (`BlackboardComponent.SetValueAsBool` _returnvalue_2 "HaveTarget" false))

(fn `UserConstructionScript`)