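; Farm plot actor that the player digs, tills and seeds, unless polluted, to spawn a BP_Crop or BP_Tree by seed ID.
; Overlaps set BP_Char's current target; InteractPlot advances stage flags behind a farming montage, with digging on a timer that spawns an accuracy-test event at a random second.
; Stages drive icons, rock/grass visibility and collision; DisplayStage refreshes every plot and crop in the world.
; Crop and tree reset functions reopen the plot.
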(event `self.ReceiveBeginPlay`
  (`self.StageSelector`)
  (`self.AdjustComponentByStage`))

(event `self.collision.OnComponentBeginOverlap`
  (params (OverlappedComponent :type "PrimitiveComponent Object Reference") (OtherActor :type "Actor Object Reference") (OtherComp :type "PrimitiveComponent Object Reference") (OtherBodyIndex :type Integer) (bFromSweep :type Boolean) (SweepResult :type "HitResult Structure (by ref)"))
  ;[1 1 1] add beginoverlap actor to currentoverlap&overlaparray
  (bind _asbp_char (cast `/Game/30DH/Character/BP_Char` OtherActor))
  (set `/Game/30DH/Character/BP_Char.CurrentOverlapObj` self _asbp_char)
  (`KismetArrayLibrary.Array_AddUnique` (`/Game/30DH/Character/BP_Char.OverlapObjArray` _asbp_char) self)
  (`self.DisplayStage`)
  (`/Game/30DH/Character/BP_Char.DisplayObjOutline` _asbp_char))

(event `self.collision.OnComponentEndOverlap`
  (params (OverlappedComponent :type "PrimitiveComponent Object Reference") (OtherActor :type "Actor Object Reference") (OtherComp :type "PrimitiveComponent Object Reference") (OtherBodyIndex :type Integer))
  (bind _asbp_char (cast `/Game/30DH/Character/BP_Char` OtherActor))
  (bind _overlapobjarray (`/Game/30DH/Character/BP_Char.OverlapObjArray` _asbp_char))
  ;[1 1 1] Remove endoverlaptrigger from overlaparray
  (`KismetArrayLibrary.Array_Remove` _overlapobjarray (`KismetArrayLibrary.Array_Find` _overlapobjarray self))
  ;[1 1 1] Check Currentoverlap == endoverlaptrigger?
  (if (== (`/Game/30DH/Character/BP_Char.CurrentOverlapObj` _asbp_char) self)
    ;[1 1 1] Check still have overlap in overlaparray?
    (if (`KismetArrayLibrary.Array_IsEmpty` _overlapobjarray)
      ;[1 1 1] if array empty -> currentoverlap = empty too
      (set `/Game/30DH/Character/BP_Char.CurrentOverlapObj` null _asbp_char)
      (else
        ;[1 1 1] if array not empty -> set currentoverlap = last obj in array
        (set `/Game/30DH/Character/BP_Char.CurrentOverlapObj` (`|GetArrayItem` _overlapobjarray (`KismetArrayLibrary.Array_LastIndex` _overlapobjarray)) _asbp_char)))
    (`/Game/30DH/Character/BP_Char.DisplayObjOutline` _asbp_char)
    (`self.DisplayStage`)))

(event `InteractPlot`
  (bind _returnvalue (`GameplayStatics.GetPlayerController` 0))
  (if (not (`self.IsPollutedPlot`))
    (bind _returnvalue_2 (`GameplayStatics.GetActorOfClass` "/Game/30DH/Character/BP_Char.BP_Char_C"))
    (if (or (`/Game/30DH/Character/BP_Char.TimeOut` _returnvalue_2) (`self.isMakingPlot`))
      _
      (elif (and (== (`/Game/30DH/Character/BP_Char.Seed` _returnvalue_2) 11) (`self.TillSoilCheck`) (not (`self.SeedPlantCheck`)))
        (`GameplayStatics.PlaySound2D` "/Game/Interface_And_Item_Sounds/WAV/Back_Click_10.Back_Click_10" 1.0 1.0 0.0 null null)
        (elif (`self.MakePlotCheck`)
          ;[1 1 1] Seed&Water: disableinput -> playmontage -> delay -> enableinput
          (`GameplayStatics.PlaySound2D` "/Game/Interface_And_Item_Sounds/WAV/Flick_Switch_01.Flick_Switch_01" 1.0 1.0 0.0 null null)
          (bind _returnvalue_3 (`GameplayStatics.GetActorOfClass` "/Game/30DH/Character/BP_Char.BP_Char_C"))
          (`self.DisableInput` _returnvalue_3 _returnvalue)
          (bind _mesh (`Character.Mesh` _returnvalue_3))
          (`|PlayMontage` _mesh "/Game/30DH/Character/Anim/Animation_farm.Animation_farm"
            (:`then`
              (`KismetSystemLibrary.Delay` 2.3)
              (`AnimInstance.Montage_Stop` (`SkeletalMeshComponent.GetAnimInstance` _mesh) 0.2 "/Game/30DH/Character/Anim/Animation_farm.Animation_farm")
              (`self.EnableInput` _returnvalue_3 _returnvalue)
              (if (`self.TillSoilCheck`)
                (if (not (`self.SeedPlantCheck`))
                  (`self.SeedPlant`)
                  (`self.StageSelector` :!label _label)
                  (`self.AdjustComponentByStage`)
                  (`GameplayStatics.PlaySound2D` "/Game/Interface_And_Item_Sounds/WAV/Coins_05.Coins_05" 1.0 1.0 0.0 null null))
                (else
                  (`self.TillSoil`)
                  (goto _label)))))
          (else
            ;[1 1 1] MakePlot: disableinput -> playmontage -> delay -> enableinput
            (`GameplayStatics.PlaySound2D` "/Game/Interface_And_Item_Sounds/WAV/Flick_Switch_01.Flick_Switch_01" 1.0 1.0 0.0 null null)
            (set `self.isMakingPlot` true)
            (bind _returnvalue_4 (`GameplayStatics.GetActorOfClass` "/Game/30DH/Character/BP_Char.BP_Char_C"))
            (`CharacterMovementComponent.DisableMovement` (`Character.CharacterMovement` _returnvalue_4))
            (`|PlayMontage` (`Character.Mesh` _returnvalue_4) "/Game/30DH/Character/Anim/Animation_farm.Animation_farm"
              (:`then`
                (set `self.SpawnEVTime` (`KismetMathLibrary.Conv_IntToDouble` (`KismetMathLibrary.RandomIntegerInRange` 2 5)))
                (`self.StartTimer`)))))))))

(event `StartTimer`
  (bind _returnvalue (`KismetSystemLibrary.K2_SetTimerDelegate` (delegate `Time++`) 1.0 true))
  (set `self.MakePlotDelay` _returnvalue))

(event `Time++`
  (bind _output_get (set `self.Second` (+ (`self.Second`) 1.0)))
  (if (== _output_get (`self.SpawnEVTime`))
    (bind _returnvalue (`|SpawnActorFromClass` "/Game/30DH/Event/EV_AccuracyTestPlot.EV_AccuracyTestPlot_C" (`self.GetTransform`) "Undefined" "MultiplyWithRoot" null null))
    (set `/Game/30DH/Event/EV_AccuracyTestPlot.Plot` self _returnvalue))
  (if (>= (`self.Second`) (`self.MaxDelay`))
    (`self.TimerFinish`)
    ;[1 1 1] MakePlot: disableinput -> playmontage -> delay -> enableinput
    (`AnimInstance.Montage_Stop` (`SkeletalMeshComponent.GetAnimInstance` (`Character.Mesh` (stale `InteractPlot` _returnvalue_4))) 0.2 "/Game/30DH/Character/Anim/Animation_farm.Animation_farm")
    (`CharacterMovementComponent.SetMovementMode` (`Character.CharacterMovement` (stale `InteractPlot` _returnvalue_4)) "MOVE_Walking" 0)
    (`self.MakePlot`)
    (set `self.isMakingPlot` false)
    (goto _label)))

(event `TimerFinish`
  (`KismetSystemLibrary.K2_ClearAndInvalidateTimerHandle` (`self.MakePlotDelay`))
  (set `self.Second` 0.0))

(fn `AdjustComponentByStage`
  (if (`self.MakePlotCheck`)
    (`SceneComponent.SetVisibility` (`self.Rock1`) false false)
    (`SceneComponent.SetVisibility` (`self.Rock2`) false false)
    (`SceneComponent.SetVisibility` (`self.Rock3`) false false)
    (if (`self.TillSoilCheck`)
      (`SceneComponent.SetVisibility` (`self.Grass1`) false false)
      (`SceneComponent.SetVisibility` (`self.Grass2`) false false)
      (`SceneComponent.SetVisibility` (`self.Grass4`) false false)
      (`SceneComponent.SetVisibility` (`self.Grass3`) false false)
      (else
        (`SceneComponent.SetVisibility` (`self.Grass1`) true false :!label _label)
        (`SceneComponent.SetVisibility` (`self.Grass2`) true false)
        (`SceneComponent.SetVisibility` (`self.Grass4`) true false)
        (`SceneComponent.SetVisibility` (`self.Grass3`) true false)))
    (else
      (`SceneComponent.SetVisibility` (`self.Rock1`) true false)
      (`SceneComponent.SetVisibility` (`self.Rock2`) true false)
      (`SceneComponent.SetVisibility` (`self.Rock3`) true false)
      (goto _label))))

(fn `AdjustPlotWhenWater`
  (params (Watering :type Boolean))
  (bind _plotmesh (`self.PlotMesh`))
  (if Watering
    (`PrimitiveComponent.SetMaterial` _plotmesh 0 "/Game/PolygonFarm/Materials/WateringPlot.WateringPlot")
    (elif (`self.IsPollutedPlot`)
      (`PrimitiveComponent.SetMaterial` _plotmesh 0 "/Game/PolygonFarm/Materials/DeadMat.DeadMat")
      (else
        (`PrimitiveComponent.SetMaterial` _plotmesh 0 "/Game/PolygonFarm/Materials/M_PolygonFarm_01_A.M_PolygonFarm_01_A")))))

(fn `ChangePlotMat`
  (if (`self.IsPollutedPlot`)
    (`PrimitiveComponent.SetMaterial` (`self.PlotMesh`) 0 "/Game/PolygonFarm/Materials/DeadMat.DeadMat")
    (else
      (`PrimitiveComponent.SetMaterial` (`self.PlotMesh`) 0 "/Game/PolygonFarm/Materials/M_PolygonFarm_01_A.M_PolygonFarm_01_A"))))

(fn `DisplayStage`
  (`|ExecutionSequence`
    (:`then_0`
      ;[1 1 1] displaystage of plot
      (bind _outactors (`GameplayStatics.GetAllActorsOfClass` "BP_Plot_C"))
      (for _array_element _outactors
        (bind _stageicon (`/Game/30DH/Farm/BP_Plot.StageIcon` _array_element))
        ;;[1 1 1] Set each stage of plot to sprite
        (`BillboardComponent.SetSprite` _stageicon (`/Game/30DH/Farm/BP_Plot.NowStageIcon` _array_element))
        (`SceneComponent.SetVisibility` _stageicon false false)
        ;;[1 1 1] check stage that alway display
        (if (or (`/Game/30DH/Farm/BP_Plot.MakePlotCheck` _array_element) (`/Game/30DH/Farm/BP_Plot.TillSoilCheck` _array_element))
          (`SceneComponent.SetVisibility` _stageicon true false)
          (else
            (bind _returnvalue (`GameplayStatics.GetActorOfClass` "/Game/30DH/Character/BP_Char.BP_Char_C"))
            ;;[1 1 1] check actor that is hovering
            (if (== (`/Game/30DH/Character/BP_Char.CurrentOverlapObj` _returnvalue) _array_element)
              (`SceneComponent.SetVisibility` _stageicon true false)
              (else
                (`SceneComponent.SetVisibility` _stageicon false false)))))))
    (:`then_1`
      ;[1 1 1] displaystage of crop
      (bind _outactors_2 (`GameplayStatics.GetAllActorsOfClass` "/Game/30DH/Farm/BP_Crop.BP_Crop_C"))
      (for _array_element_2 _outactors_2
        (if (`/Game/30DH/Farm/BP_Crop.CuttingStage` _array_element_2)
          ;;[1 1 1] romove
          (`SceneComponent.SetVisibility` (`/Game/30DH/Farm/BP_Crop.FertilizeWidget` _array_element_2) false false)
          (bind _stageicon_2 (`/Game/30DH/Farm/BP_Crop.StageIcon` _array_element_2))
          (`SceneComponent.SetVisibility` _stageicon_2 false false)
          (set `BillboardComponent.Sprite` "/Game/30DH/Farm/StageIcon/uproot.uproot" _stageicon_2)
          (`SceneComponent.SetVisibility` _stageicon_2 true false)
          (else
            (`|ExecutionSequence`
              (:`then_0`
                (bind _stageicon_3 (`/Game/30DH/Farm/BP_Crop.StageIcon` _array_element_2))
                ;;[1 1 1] Set each stage of plot to sprite
                (`BillboardComponent.SetSprite` _stageicon_3 (`/Game/30DH/Farm/BP_Crop.NowStageIcon` _array_element_2))
                (`SceneComponent.SetVisibility` _stageicon_3 false false)
                ;;[1 1 1] chek stage display by hovering only
                (if (and (`/Game/30DH/Farm/BP_Crop.WateringCheck` _array_element_2) (`/Game/30DH/Farm/BP_Crop.EnvironmentSuitableCheck` _array_element_2) (not (`/Game/30DH/Farm/BP_Crop.FullyGrownCheck` _array_element_2)) (`/Game/30DH/Farm/BP_Crop.NotInsectedCheck` _array_element_2) (not (`/Game/30DH/Farm/BP_Crop.IsDead` _array_element_2)))
                  (bind _returnvalue_2 (`GameplayStatics.GetActorOfClass` "/Game/30DH/Character/BP_Char.BP_Char_C"))
                  ;;[1 1 1] check actor that is hovering
                  (if (== (`/Game/30DH/Character/BP_Char.CurrentOverlapObj` _returnvalue_2) _array_element_2)
                    (`SceneComponent.SetVisibility` _stageicon_3 true false)
                    (bind _fertilizewidget (`/Game/30DH/Farm/BP_Crop.FertilizeWidget` _array_element_2))
                    (`SceneComponent.SetVisibility` _fertilizewidget true false)
                    (else
                      (`SceneComponent.SetVisibility` _stageicon_3 false false)
                      (`SceneComponent.SetVisibility` _fertilizewidget false false)))
                  (else
                    (`SceneComponent.SetVisibility` _stageicon_3 true false)
                    (`SceneComponent.SetVisibility` _fertilizewidget false false))))
              (:`then_1`
                ;[1 1 1] set visibility to show only hover crop
                (bind _outactors_3 (`GameplayStatics.GetAllActorsOfClass` "/Game/30DH/Farm/BP_Crop.BP_Crop_C"))
                (for _array_element_3 _outactors_3
                  (`/Engine/EditorBlueprintResources/StandardMacros.IsValid` (`/Game/30DH/Farm/BP_Crop.WB_CropInfo` _array_element_3)
                    (:`Is Valid`
                      (bind _returnvalue_3 (`GameplayStatics.GetActorOfClass` "/Game/30DH/Character/BP_Char.BP_Char_C"))
                      (if (== (`/Game/30DH/Character/BP_Char.CurrentOverlapObj` _returnvalue_3) _array_element_3)
                        (bind _wb_cropinfo (`/Game/30DH/Farm/BP_Crop.WB_CropInfo` _array_element_3))
                        (bind _aswb_crop_info (cast `/Game/30DH/Farm/Widget/WB_CropInfo` _wb_cropinfo))
                        (set `Widget.Visibility` "Visible" _aswb_crop_info)
                        (else
                          (bind _aswb_crop_info_2 (cast `/Game/30DH/Farm/Widget/WB_CropInfo` _wb_cropinfo))
                          (set `Widget.Visibility` "Hidden" _aswb_crop_info_2))))))))))))))

(fn `MakePlot`
  (set `self.MakePlotCheck` true))

(fn `ResetFromCrop`
  (set `self.MakePlotCheck` true)
  (set `self.TillSoilCheck` false)
  (set `self.SeedPlantCheck` false)
  (`PrimitiveComponent.SetCollisionProfileName` (`self.collision`) "OverlapAllDynamic" true)
  (`self.StageSelector`)
  (`self.AdjustComponentByStage`))

(fn `ResetFromTree`
  (set `self.MakePlotCheck` false)
  (set `self.TillSoilCheck` false)
  (set `self.SeedPlantCheck` false)
  (`PrimitiveComponent.SetCollisionProfileName` (`self.collision`) "OverlapAllDynamic" true)
  (`self.StageSelector`)
  (`self.AdjustComponentByStage`))

(fn `SeedPlant`
  (bind _returnvalue (`KismetMathLibrary.MakeTransform` (`KismetMathLibrary.MakeVector` (.x (`SceneComponent.K2_GetComponentLocation` (`self.PlotMesh`))) (.y (`SceneComponent.K2_GetComponentLocation` (`self.PlotMesh`))) (+ (.z (`SceneComponent.K2_GetComponentLocation` (`self.PlotMesh`))) 30.0))))
  (bind _returnvalue_2 (`GameplayStatics.GetActorOfClass` "/Game/30DH/Character/BP_Char.BP_Char_C"))
  (if (not (== (`/Game/30DH/Character/BP_Char.Seed` _returnvalue_2) 11))
    (if (<= (`/Game/30DH/Character/BP_Char.Seed` _returnvalue_2) 5)
      (bind _returnvalue_3 (`|SpawnActorFromClass` "/Game/30DH/Farm/BP_Crop.BP_Crop_C" _returnvalue "Undefined" "MultiplyWithRoot" null null))
      (bind _seed (`/Game/30DH/Character/BP_Char.Seed` _returnvalue_2))
      (`/Game/30DH/Farm/BP_Crop.InitializeCrop` _returnvalue_3 _seed)
      (set `/Game/30DH/Farm/BP_Crop.PlantedTile` self _returnvalue_3)
      (`PrimitiveComponent.SetCollisionProfileName` (`self.collision`) "NoCollision" true)
      (set `self.SeedPlantCheck` true)
      (`/Game/30DH/Character/BP_Char.DisplayObjOutline` _returnvalue_2)
      (`/Game/30DH/Farm/BP_Crop.DisplayStage` _returnvalue_3)
      (else
        (bind _returnvalue_4 (`|SpawnActorFromClass` "/Game/30DH/Farm/BP_Tree.BP_Tree_C" _returnvalue "Undefined" "MultiplyWithRoot" null null))
        (`/Game/30DH/Farm/BP_Tree.InitializeTree` _returnvalue_4 _seed)
        (set `/Game/30DH/Farm/BP_Tree.PlantedTileTree` self _returnvalue_4)
        (`PrimitiveComponent.SetCollisionProfileName` (`self.collision`) "NoCollision" true)
        (set `self.SeedPlantCheck` true)
        (`/Game/30DH/Character/BP_Char.DisplayObjOutline` _returnvalue_2)))
    (bind _returnvalue_5 (`GameplayStatics.GetActorOfClass` "/Game/30DH/Event/AnimalEvent/BP_Mole.BP_Mole_C"))
    (`/Engine/EditorBlueprintResources/StandardMacros.IsValid` _returnvalue_5
      (:`Is Valid`
        (if (== (`BlackboardComponent.GetValueAsObject` (`AIBlueprintHelperLibrary.GetBlackboard` (`AIBlueprintHelperLibrary.GetAIController` _returnvalue_5)) "Target") self)
          (`/Game/30DH/Event/AnimalEvent/BP_Mole.ResetFromTargetDestroyed` _returnvalue_5))))))

(fn `StageSelector`
  (if (not (`self.IsPollutedPlot`))
    (if (`self.MakePlotCheck`)
      (if (`self.TillSoilCheck`)
        (if (`self.SeedPlantCheck`)
          (set `self.NowStageIcon` null)
          (else
            (set `self.NowStageIcon` "/Game/30DH/Farm/StageIcon/seed.seed")))
        (else
          (set `self.NowStageIcon` "/Game/30DH/Farm/StageIcon/till.till")))
      (else
        (set `self.NowStageIcon` "/Game/30DH/Farm/StageIcon/dig.dig")))
    (else
      (set `self.NowStageIcon` null)))
  (`self.DisplayStage`)
  (`self.AdjustComponentByStage`))

(fn `TillSoil`
  (set `self.TillSoilCheck` true))

(fn `UserConstructionScript`)