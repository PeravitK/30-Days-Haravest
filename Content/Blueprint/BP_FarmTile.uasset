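; Farm tile actor that registers with the player on overlap and plants the crop or tree chosen by the character's Seed.
; Crops swap meshes through three stages on a Text3D countdown macro, with a small chance of insects halting the second.
; Trees and cactus finish instantly as one mesh.
; Activate harvests grown plants, spawning only wheat or corn pickups (most crops yield corn), while Cut clears the tile with the axe.
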(event `PlantLettuce`
  ;[0.4004 1 0.2741] Crop
  ;;[1 1 1] Lettuce Growing state
  (if (`self.IsOverlap`)
    (if (`self.IsFullyGrown?`)
      _
      (elif (not (`self.IsSomethingPlanted`))
        (set `self.IsSomethingPlanted` true)
        (bind _returnvalue (`AddComponent|NODE_AddStaticMeshComponent-18`))
        (`PrimitiveComponent.SetCollisionProfileName` _returnvalue "NoCollision" true)
        (`self.GrowTime` (`self.WheatGrowTime`)
          (:`Out`
            (`ActorComponent.K2_DestroyComponent` _returnvalue)
            (bind _returnvalue_2 (`AddComponent|NODE_AddStaticMeshComponent-19`))
            (`PrimitiveComponent.SetCollisionProfileName` _returnvalue_2 "NoCollision" true)
            (`self.GrowTime` (`self.WheatGrowTime`)
              (:`Out`
                (`self.ChanceOfInsect` _returnvalue_2
                  (:`No Insect`
                    (`ActorComponent.K2_DestroyComponent` _returnvalue_2)
                    (bind _returnvalue_3 (`AddComponent|NODE_AddStaticMeshComponent-20`))
                    (`PrimitiveComponent.SetCollisionProfileName` _returnvalue_3 "NoCollision" true)
                    (set `self.IsFullyGrown?` true)
                    (set `self.Current Mesh` _returnvalue_3)
                    (set `self.WhatCanBeHarvest` "Corn")))))))))))

(event `self.Box.OnComponentBeginOverlap`
  (params (OverlappedComponent :type "PrimitiveComponent Object Reference") (OtherActor :type "Actor Object Reference") (OtherComp :type "PrimitiveComponent Object Reference") (OtherBodyIndex :type Integer) (bFromSweep :type Boolean) (SweepResult :type "HitResult Structure (by ref)"))
  ;[1 1 1] Checking Overlap
  (set `self.IsOverlap` true)
  (bind _asbp_third_person_character (cast `/Game/ThirdPerson/Blueprints/BP_ThirdPersonCharacter` (`GameplayStatics.GetPlayerPawn` 0)))
  (set `/Game/ThirdPerson/Blueprints/BP_ThirdPersonCharacter.FarmTile_BP` self _asbp_third_person_character)
  (`KismetSystemLibrary.PrintString` "Overlap!" true true (struct :`R` 1.0 :`B` 0.088833 :`A` 1.0)))

(event `PlantCactus`
  ;[0.3316 1 0.8968] Tree
  ;;[1 1 1] Cuctus state
  (if (`self.IsOverlap`)
    (if (`self.IsFullyGrown?`)
      _
      (elif (not (`self.IsSomethingPlanted`))
        (set `self.IsSomethingPlanted` true)
        (bind _returnvalue (`AddComponent|NODE_AddStaticMeshComponent-33`))
        (`PrimitiveComponent.SetCollisionProfileName` _returnvalue "NoCollision" true)
        (set `self.IsFullyGrown?` true)
        (set `self.Current Mesh` null)))))

(event `self.Box.OnComponentEndOverlap`
  (params (OverlappedComponent :type "PrimitiveComponent Object Reference") (OtherActor :type "Actor Object Reference") (OtherComp :type "PrimitiveComponent Object Reference") (OtherBodyIndex :type Integer))
  ;[1 1 1] Checking Overlap
  (set `self.IsOverlap` false))

(event `PlantStrawberry`
  ;[0.4004 1 0.2741] Crop
  ;;[1 1 1] Strawberry Growing state
  (if (`self.IsOverlap`)
    (if (`self.IsFullyGrown?`)
      _
      (elif (not (`self.IsSomethingPlanted`))
        (set `self.IsSomethingPlanted` true)
        (bind _returnvalue (`AddComponent|NODE_AddStaticMeshComponent-12`))
        (`PrimitiveComponent.SetCollisionProfileName` _returnvalue "NoCollision" true)
        (`self.GrowTime` (`self.WheatGrowTime`)
          (:`Out`
            (`ActorComponent.K2_DestroyComponent` _returnvalue)
            (bind _returnvalue_2 (`AddComponent|NODE_AddStaticMeshComponent-13`))
            (`PrimitiveComponent.SetCollisionProfileName` _returnvalue_2 "NoCollision" true)
            (`self.GrowTime` (`self.WheatGrowTime`)
              (:`Out`
                (`self.ChanceOfInsect` _returnvalue_2
                  (:`No Insect`
                    (`ActorComponent.K2_DestroyComponent` _returnvalue_2)
                    (bind _returnvalue_3 (`AddComponent|NODE_AddStaticMeshComponent-14`))
                    (`PrimitiveComponent.SetCollisionProfileName` _returnvalue_3 "NoCollision" true)
                    (set `self.IsFullyGrown?` true)
                    (set `self.Current Mesh` _returnvalue_3)
                    (set `self.WhatCanBeHarvest` "Corn")))))))))))

(event `PlantLvory`
  ;[0.3316 1 0.8968] Tree
  ;;[1 1 1] Lvory state
  (if (`self.IsOverlap`)
    (if (`self.IsFullyGrown?`)
      _
      (elif (not (`self.IsSomethingPlanted`))
        (set `self.IsSomethingPlanted` true)
        (bind _returnvalue (`AddComponent|NODE_AddStaticMeshComponent-35`))
        (`PrimitiveComponent.SetCollisionProfileName` _returnvalue "NoCollision" true)
        (set `self.IsFullyGrown?` true)
        (set `self.Current Mesh` null)))))

(event `PlantTomato`
  ;[0.4004 1 0.2741] Crop
  ;;[1 1 1] Tomato Growing state
  (if (`self.IsOverlap`)
    (if (`self.IsFullyGrown?`)
      _
      (elif (not (`self.IsSomethingPlanted`))
        (set `self.IsSomethingPlanted` true)
        (bind _returnvalue (`AddComponent|NODE_AddStaticMeshComponent-9`))
        (`PrimitiveComponent.SetCollisionProfileName` _returnvalue "NoCollision" true)
        (`self.GrowTime` (`self.WheatGrowTime`)
          (:`Out`
            (`ActorComponent.K2_DestroyComponent` _returnvalue)
            (bind _returnvalue_2 (`AddComponent|NODE_AddStaticMeshComponent-10`))
            (`PrimitiveComponent.SetCollisionProfileName` _returnvalue_2 "NoCollision" true)
            (`self.GrowTime` (`self.WheatGrowTime`)
              (:`Out`
                (`self.ChanceOfInsect` _returnvalue_2
                  (:`No Insect`
                    (`ActorComponent.K2_DestroyComponent` _returnvalue_2)
                    (bind _returnvalue_3 (`AddComponent|NODE_AddStaticMeshComponent-11`))
                    (`PrimitiveComponent.SetCollisionProfileName` _returnvalue_3 "NoCollision" true)
                    (set `self.IsFullyGrown?` true)
                    (set `self.Current Mesh` _returnvalue_3)
                    (set `self.WhatCanBeHarvest` "Corn")))))))))))

(event `PlantPine`
  ;[0.3316 1 0.8968] Tree
  ;;[1 1 1] Pine state
  (if (`self.IsOverlap`)
    (if (`self.IsFullyGrown?`)
      _
      (elif (not (`self.IsSomethingPlanted`))
        (set `self.IsSomethingPlanted` true)
        (bind _returnvalue (`AddComponent|NODE_AddStaticMeshComponent-36`))
        (`PrimitiveComponent.SetCollisionProfileName` _returnvalue "NoCollision" true)
        (set `self.IsFullyGrown?` true)
        (set `self.Current Mesh` null)
        (set `self.WhatCanBeHarvest` "Corn")))))

(event `PlantPotato`
  ;[0.4004 1 0.2741] Crop
  ;;[1 1 1] Potato Growing state
  (if (`self.IsOverlap`)
    (if (`self.IsFullyGrown?`)
      _
      (elif (not (`self.IsSomethingPlanted`))
        (set `self.IsSomethingPlanted` true)
        (bind _returnvalue (`AddComponent|NODE_AddStaticMeshComponent-6`))
        (`PrimitiveComponent.SetCollisionProfileName` _returnvalue "NoCollision" true)
        (`self.GrowTime` (`self.WheatGrowTime`)
          (:`Out`
            (`ActorComponent.K2_DestroyComponent` _returnvalue)
            (bind _returnvalue_2 (`AddComponent|NODE_AddStaticMeshComponent-7`))
            (`PrimitiveComponent.SetCollisionProfileName` _returnvalue_2 "NoCollision" true)
            (`self.GrowTime` (`self.WheatGrowTime`)
              (:`Out`
                (`self.ChanceOfInsect` _returnvalue_2
                  (:`No Insect`
                    (`ActorComponent.K2_DestroyComponent` _returnvalue_2)
                    (bind _returnvalue_3 (`AddComponent|NODE_AddStaticMeshComponent-8`))
                    (`PrimitiveComponent.SetCollisionProfileName` _returnvalue_3 "NoCollision" true)
                    (set `self.IsFullyGrown?` true)
                    (set `self.Current Mesh` _returnvalue_3)
                    (set `self.WhatCanBeHarvest` "Corn")))))))))))

(event `PlantMaple`
  ;[0.3316 1 0.8968] Tree
  ;;[1 1 1] Maple state
  (if (`self.IsOverlap`)
    (if (`self.IsFullyGrown?`)
      _
      (elif (not (`self.IsSomethingPlanted`))
        (set `self.IsSomethingPlanted` true)
        (bind _returnvalue (`AddComponent|NODE_AddStaticMeshComponent-37`))
        (`PrimitiveComponent.SetCollisionProfileName` _returnvalue "NoCollision" true)
        (set `self.IsFullyGrown?` true)
        (set `self.Current Mesh` null)
        (set `self.WhatCanBeHarvest` "Corn")))))

(event `PlantCorn`
  ;[0.4004 1 0.2741] Crop
  ;;[1 1 1] Corn Growing state
  (if (`self.IsOverlap`)
    (if (`self.IsFullyGrown?`)
      _
      (elif (not (`self.IsSomethingPlanted`))
        (set `self.IsSomethingPlanted` true)
        (bind _returnvalue (`AddComponent|NODE_AddStaticMeshComponent-3`))
        (`PrimitiveComponent.SetCollisionProfileName` _returnvalue "NoCollision" true)
        (`self.GrowTime` (`self.WheatGrowTime`)
          (:`Out`
            (`ActorComponent.K2_DestroyComponent` _returnvalue)
            (bind _returnvalue_2 (`AddComponent|NODE_AddStaticMeshComponent-4`))
            (`PrimitiveComponent.SetCollisionProfileName` _returnvalue_2 "NoCollision" true)
            (`self.GrowTime` (`self.WheatGrowTime`)
              (:`Out`
                (`self.ChanceOfInsect` _returnvalue_2
                  (:`No Insect`
                    (`ActorComponent.K2_DestroyComponent` _returnvalue_2)
                    (bind _returnvalue_3 (`AddComponent|NODE_AddStaticMeshComponent-5`))
                    (`PrimitiveComponent.SetCollisionProfileName` _returnvalue_3 "NoCollision" true)
                    (set `self.IsFullyGrown?` true)
                    (set `self.Current Mesh` _returnvalue_3)
                    (set `self.WhatCanBeHarvest` "Corn")))))))))))

(event `PlantOak`
  ;[0.3316 1 0.8968] Tree
  ;;[1 1 1] Oak
  (if (`self.IsOverlap`)
    (if (`self.IsFullyGrown?`)
      _
      (elif (not (`self.IsSomethingPlanted`))
        (set `self.IsSomethingPlanted` true)
        (bind _returnvalue (`AddComponent|NODE_AddStaticMeshComponent-38`))
        (`PrimitiveComponent.SetCollisionProfileName` _returnvalue "NoCollision" true)
        (set `self.IsFullyGrown?` true)
        (set `self.Current Mesh` null)
        (set `self.WhatCanBeHarvest` "Corn")))))

(event `self.ReceiveBeginPlay`
  (set `Text3DComponent.Text` (`self.Value`) (`self.Text3D`)))

(event `Plant Wheat`
  ;[1 1 1] Wheat Growing state
  (if (`self.IsOverlap`)
    (if (`self.IsFullyGrown?`)
      _
      (elif (not (`self.IsSomethingPlanted`))
        (set `self.IsSomethingPlanted` true)
        (set `self.IsFullyGrown?` false)
        (bind _returnvalue (`AddComponent|NODE_AddStaticMeshComponent-0`))
        (`PrimitiveComponent.SetCollisionProfileName` _returnvalue "NoCollision" true)
        (set `self.Current Mesh` _returnvalue)
        (`self.GrowTime` (`self.WheatGrowTime`)
          (:`Out`
            (if (`self.IsSomethingPlanted`)
              (`ActorComponent.K2_DestroyComponent` _returnvalue)
              (bind _returnvalue_2 (`AddComponent|NODE_AddStaticMeshComponent-1`))
              (`PrimitiveComponent.SetCollisionProfileName` _returnvalue_2 "NoCollision" true)
              (set `self.Current Mesh` _returnvalue_2)
              (`self.GrowTime` (`self.WheatGrowTime`)
                (:`Out`
                  (if (`self.IsSomethingPlanted`)
                    (`self.ChanceOfInsect` _returnvalue_2
                      (:`No Insect`
                        (`ActorComponent.K2_DestroyComponent` _returnvalue_2)
                        (set `self.Current Mesh` _returnvalue_2)
                        (if (`self.IsSomethingPlanted`)
                          (bind _returnvalue_3 (`AddComponent|NODE_AddStaticMeshComponent-2`))
                          (`PrimitiveComponent.SetCollisionProfileName` _returnvalue_3 "NoCollision" true)
                          (set `self.IsFullyGrown?` true)
                          (set `self.Current Mesh` _returnvalue_3)
                          (set `self.WhatCanBeHarvest` "Wheat"))))))))))))))

(event `/Game/Blueprint/BPI_Activate.Activate`
  ;[1 1 1] Can Harvest?
  (if (`self.IsOverlap`)
    (if (`self.IsFullyGrown?`)
      (if (`self.IsSomethingPlanted`)
        (`self.Harvesting`)
        (`KismetSystemLibrary.Delay` 0.2)
        (set `self.IsFullyGrown?` false)
        (set `self.Current Mesh` null)
        (set `self.IsSomethingPlanted` false)
        (set `self.WhatCanBeHarvest` "")))))

(event `/Game/Blueprint/BPI_PlantSeed.PlantSeed`
  ;[1 1 1] Checking select seed
  (if (not (`self.IsSomethingPlanted`))
    (bind _asbp_third_person_character (cast `/Game/ThirdPerson/Blueprints/BP_ThirdPersonCharacter` (`GameplayStatics.GetPlayerCharacter` 0)))
    (switch `int` (`/Game/ThirdPerson/Blueprints/BP_ThirdPersonCharacter.Seed` _asbp_third_person_character)
      (:`0`
        (`self.Plant Wheat`))
      (:`1`
        (`self.PlantPotato`))
      (:`2`
        (`self.PlantCorn`))
      (:`3`
        (`self.PlantTomato`))
      (:`4`
        (`self.PlantStrawberry`))
      (:`5`
        (`self.PlantLettuce`))
      (:`6`
        (`self.PlantLvory`))
      (:`7`
        (`self.PlantCactus`))
      (:`8`
        (`self.PlantPine`))
      (:`9`
        (`self.PlantMaple`))
      (:`10`
        (`self.PlantOak`)))
    (set `self.IsSomethingPlanted` true)))

(event `/Game/Blueprint/BPI_Cut.Cut`
  ;[1 1 1] Cutting
  (bind _asbp_third_person_character (cast `/Game/ThirdPerson/Blueprints/BP_ThirdPersonCharacter` (`GameplayStatics.GetPlayerCharacter` 0)))
  (switch `int` (`/Game/ThirdPerson/Blueprints/BP_ThirdPersonCharacter.Seed` _asbp_third_person_character)
    (:`11`
      (set `self.SelectAxe` true)
      (`ActorComponent.K2_DestroyComponent` (`self.Current Mesh`))
      (set `self.IsSomethingPlanted` false)
      (set `self.Time` 0)
      (set `self.IsFullyGrown?` false)
      (`SceneComponent.SetVisibility` (`self.Text3D`) false false))))

(fn `Harvesting`
  (bind _current_mesh (`self.Current Mesh`))
  (bind _returnvalue (`KismetMathLibrary.Conv_VectorToTransform` (`SceneComponent.K2_GetComponentLocation` (`self.Text3D`))))
  ;[1 1 1] Harvesting (destory crop)
  (if (`self.IsFullyGrown?`)
    (`/Engine/EditorBlueprintResources/StandardMacros.IsValid` _current_mesh
      (:`Is Valid`
        (`ActorComponent.K2_DestroyComponent` _current_mesh)
        (switch `string` (`self.WhatCanBeHarvest`)
          (:`Wheat`
            (`|SpawnActorFromClass` "/Game/Blueprint/BP_WheatLoose.BP_WheatLoose_C" _returnvalue "Undefined" "MultiplyWithRoot" null null))
          (:`Corn`
            (`|SpawnActorFromClass` "/Game/Blueprint/BP_CornLoose.BP_CornLoose_C" _returnvalue "Undefined" "MultiplyWithRoot" null null)))))))

(fn `UserConstructionScript`)