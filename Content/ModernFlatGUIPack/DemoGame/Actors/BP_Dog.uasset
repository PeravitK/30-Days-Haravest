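; BP_Dog is the wandering dog pawn of the farm demo game, killed by touching a BP_Egg or leaving the square play bounds.
; While alive, Tick repeatedly waits a short random delay and issues an AI move to a random reachable nearby point.
; Death launches its child static meshes upward as physics debris, decrements the game mode's dog count, and destroys the actor two seconds later.
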(event `self.ReceiveBeginPlay`
  (for _array_element (`SceneComponent.GetChildrenComponents` (`self.Mesh`) true)
    (bind _asstatic_mesh_component (cast `StaticMeshComponent` _array_element))
    (`KismetArrayLibrary.Array_Add` (`self.ExplodableMeshes`) _asstatic_mesh_component)))

(event `self.ReceiveTick`
  (params (DeltaSeconds :type "Float (single-precision)"))
  (`|ExecutionSequence`
    (:`then_0`
      (if (`self.IsOutOfBounds`)
        (`self.Die`)))
    (:`then_1`
      (if (`self.IsDying`)
        (bind _output_get (set `self.DyingTimeCtr` (+ (`self.DyingTimeCtr`) DeltaSeconds)))
        (if (>= _output_get 2.0)
          (`self.K2_DestroyActor`))
        (elif (not (`self.IsMoving`))
          (set `self.IsMoving` true)
          (`KismetSystemLibrary.Delay` (`KismetMathLibrary.RandomFloatInRange` 0.5 1.5))
          (bind _output_get_2 (set `self.AiMoveToPoint` (`NavigationSystemV1.K2_GetRandomReachablePointInRadius` (`self.K2_GetActorLocation`) 1000.0 null null)))
          (`|AIMoveTo` self _output_get_2 null
            (:`then`
              (set `self.IsMoving` false))))))))

(event `self.ReceiveActorBeginOverlap`
  (params (OtherActor :type "Actor Object Reference"))
  (if (`KismetMathLibrary.ClassIsChildOf` (`GameplayStatics.GetObjectClass` OtherActor) "/Game/ModernFlatGUIPack/DemoGame/Actors/BP_Egg.BP_Egg_C")
    (if (not (`self.IsDying`))
      (`self.Die`))))

(event `Die`
  (if (not (`self.IsDying`))
    (set `self.IsDying` true)
    (`|ExecutionSequence`
      (:`then_0`
        (for _array_element (`self.ExplodableMeshes`)
          (`PrimitiveComponent.SetSimulatePhysics` _array_element true)
          (`PrimitiveComponent.AddImpulse` _array_element (0.0 0.0 500.0) "None" true)))
      (:`then_1`
        (`/Game/ModernFlatGUIPack/DemoGame/Blueprints/GM_FarmGame.DecrementDog` (`/Game/ModernFlatGUIPack/DemoGame/Blueprints/BPFL_Demo.GetFarmGameMode`))))))

(fn `IsOutOfBounds`
  (returns (OutOfBounds :type Boolean))
  (locals (OutOfBoundsDistance :type "Float (double-precision)" :default 360.0))
  (bind _outofboundsdistance (`local.OutOfBoundsDistance`))
  (bind (_returnvalue_x _returnvalue_y) (`KismetMathLibrary.BreakVector` (`SceneComponent.K2_GetComponentLocation` (`self.CapsuleComponent`))))
  (bind _returnvalue (* (`local.OutOfBoundsDistance`) -1.0))
  (return (or (> _returnvalue_x _outofboundsdistance) (< _returnvalue_x _returnvalue) (> _returnvalue_y _outofboundsdistance) (< _returnvalue_y _returnvalue))))

(fn `UserConstructionScript`)