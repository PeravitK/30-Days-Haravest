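; Game mode Blueprint that switches the background music between Spring, Rainy, Summer and Winter tracks.
; A Music event passes the requested value to ChangeMusic, which switches on it to pick the track.
; Each case deactivates and destroys any current audio component, then spawns the new track as a 2D sound and stores it, with no crossfade.
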(event `Music`
  (params (Music :type "/Game/30DH/Sound/BP_Music Enum" :default "NewEnumerator4"))
  (`self.ChangeMusic` Music))

(fn `ChangeMusic`
  (params (Music :type "/Game/30DH/Sound/BP_Music Enum" :default "NewEnumerator4"))
  (switch `/Game/30DH/Sound/BP_Music` Music
    (:`NewEnumerator0`
      (if (`KismetSystemLibrary.IsValid` (`self.Sound`))
        (`ActorComponent.SetActive` (`self.Sound`) false false)
        (`ActorComponent.K2_DestroyComponent` (`self.Sound`))
        (set `self.Sound` null))
      (bind _returnvalue (`GameplayStatics.SpawnSound2D` "/Game/30DH/Sound/SpringMusic.SpringMusic" 1.0 1.0 0.0 null))
      (set `self.Sound` _returnvalue))
    (:`NewEnumerator1`
      (if (`KismetSystemLibrary.IsValid` (`self.Sound`))
        (`ActorComponent.SetActive` (`self.Sound`) false false)
        (`ActorComponent.K2_DestroyComponent` (`self.Sound`))
        (set `self.Sound` null))
      (bind _returnvalue_2 (`GameplayStatics.SpawnSound2D` "/Game/30DH/Sound/RainyMusic.RainyMusic" 1.0 1.0 0.0 null))
      (set `self.Sound` _returnvalue_2))
    (:`NewEnumerator2`
      (if (`KismetSystemLibrary.IsValid` (`self.Sound`))
        (`ActorComponent.SetActive` (`self.Sound`) false false)
        (`ActorComponent.K2_DestroyComponent` (`self.Sound`))
        (set `self.Sound` null))
      (bind _returnvalue_3 (`GameplayStatics.SpawnSound2D` "/Game/30DH/Sound/SummerMusic.SummerMusic" 1.0 1.0 0.0 null))
      (set `self.Sound` _returnvalue_3))
    (:`NewEnumerator3`
      (if (`KismetSystemLibrary.IsValid` (`self.Sound`))
        (`ActorComponent.SetActive` (`self.Sound`) false false)
        (`ActorComponent.K2_DestroyComponent` (`self.Sound`))
        (set `self.Sound` null))
      (bind _returnvalue_4 (`GameplayStatics.SpawnSound2D` "/Game/30DH/Sound/WinterMusic.WinterMusic" 1.0 1.0 0.0 null))
      (set `self.Sound` _returnvalue_4))))

(fn `UserConstructionScript`)