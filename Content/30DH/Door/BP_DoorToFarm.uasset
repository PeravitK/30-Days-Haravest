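; Interactable door that takes BP_Char to the Farm if the day's door choice is unset or already Farm.
; Collision overlaps maintain the character's overlap array, current target and outline.
; GoToFarm updates the location widget, teleports the character, locks the choice and starts the timer on first selection, blends to the farm camera and starts tree environment effects.
; Unless time is out, it also starts the animal trigger, even when travel is refused.
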(event `self.collision.OnComponentBeginOverlap`
  (params (OverlappedComponent :type "PrimitiveComponent Object Reference") (OtherActor :type "Actor Object Reference") (OtherComp :type "PrimitiveComponent Object Reference") (OtherBodyIndex :type Integer) (bFromSweep :type Boolean) (SweepResult :type "HitResult Structure (by ref)"))
  ;[1 1 1] add beginoverlap actor to currentoverlap&overlaparray
  (bind _asbp_char (cast `/Game/30DH/Character/BP_Char` OtherActor))
  (set `/Game/30DH/Character/BP_Char.CurrentOverlapObj` self _asbp_char)
  (`KismetArrayLibrary.Array_AddUnique` (`/Game/30DH/Character/BP_Char.OverlapObjArray` _asbp_char) self)
  (`/Game/30DH/Character/BP_Char.DisplayObjOutline` _asbp_char))

(event `self.collision.OnComponentEndOverlap`
  (params (OverlappedComponent :type "PrimitiveComponent Object Reference") (OtherActor :type "Actor Object Reference") (OtherComp :type "PrimitiveComponent Object Reference") (OtherBodyIndex :type Integer))
  (bind _asbp_char (cast `/Game/30DH/Character/BP_Char` OtherActor))
  (bind _overlapobjarray (`/Game/30DH/Character/BP_Char.OverlapObjArray` _asbp_char))
  (`KismetArrayLibrary.Array_Remove` _overlapobjarray (`KismetArrayLibrary.Array_Find` _overlapobjarray self))
  ;[1 1 1] Check Currentoverlap == endoverlaptrigger?
  (if (== (`/Game/30DH/Character/BP_Char.CurrentOverlapObj` _asbp_char) self)
    ;[1 1 1] Check still have overlap in overlaparray?
    (if (`KismetArrayLibrary.Array_IsEmpty` _overlapobjarray)
      ;[1 1 1] if array empty -> currentoverlap = empty too
      (set `/Game/30DH/Character/BP_Char.CurrentOverlapObj` null _asbp_char)
      (else
        ;[1 1 1] if array not empty -> set currentoverlap = last obj in array
        (set `/Game/30DH/Character/BP_Char.CurrentOverlapObj` (`|GetArrayItem` _overlapobjarray (`KismetArrayLibrary.Array_LastIndex` _overlapobjarray)) _asbp_char)))
    (`/Game/30DH/Character/BP_Char.DisplayObjOutline` _asbp_char)))

(fn `GoToFarm`
  (locals (NewLocalVar :type "TimerHandle Structure"))
  (`|ExecutionSequence`
    (:`then_0`
      (bind _returnvalue (`GameplayStatics.GetActorOfClass` "/Game/30DH/Character/BP_Char.BP_Char_C"))
      ;[1 1 1] check already select door in day?
      (if (or (`KismetStringLibrary.EqualEqual_StrStr` (`/Game/30DH/Character/BP_Char.ChooseDoor` _returnvalue) "Farm") (`KismetStringLibrary.EqualEqual_StrStr` (`/Game/30DH/Character/BP_Char.ChooseDoor` _returnvalue)))
        (`|ExecutionSequence`
          (:`then_0`
            ;[1 1 1] update widget
            (set `/Game/30DH/Character/BP_Char.CurrentLocation` "Farm" _returnvalue)
            (`/Game/30DH/Character/BP_Char.ManageWidget` _returnvalue))
          (:`then_1`
            ;[1 1 1] set character location
            (bind _returnvalue_2 (`GameplayStatics.GetActorOfClass` "/Game/30DH/Character/BP_Char.BP_Char_C"))
            (`self.K2_SetActorLocationAndRotation` _returnvalue_2 (80.0 -600.0 0.0) (struct :`Yaw` 90.0) false false))
          (:`then_2`
            ;[1 1 1] start timer & set door selection
            (bind _returnvalue_3 (`GameplayStatics.GetActorOfClass` "/Game/30DH/Character/BP_Char.BP_Char_C"))
            (if (not (`KismetStringLibrary.EqualEqual_StrStr` (`/Game/30DH/Character/BP_Char.ChooseDoor` _returnvalue_3) "Farm"))
              (bind _returnvalue_4 (`GameplayStatics.GetActorOfClass` "/Game/30DH/Environment/BP_Timecontroller.BP_Timecontroller_C"))
              (`/Game/30DH/Environment/BP_Timecontroller.StartTimer` _returnvalue_4)
              (set `/Game/30DH/Character/BP_Char.ChooseDoor` "Farm" _returnvalue_3)))
          (:`then_3`
            ;[1 1 1] set camera
            (bind _outactors (`GameplayStatics.GetAllActorsOfClass` "/Script/Engine.CameraActor"))
            (for _array_element _outactors
              (if (`KismetStringLibrary.EqualEqual_StrStr` (`KismetSystemLibrary.GetDisplayName` _array_element) "Farm_CameraActor")
                (`PlayerController.SetViewTargetWithBlend` (`PlayerState.GetPlayerController` (`Pawn.PlayerState` _returnvalue)) _array_element 0.0 "VTBlend_Linear" 0.0 false))))
          (:`then_4`
            ;[1 1 1] Reduce env stat by tree
            (bind _outactors_2 (`GameplayStatics.GetAllActorsOfClass` "/Game/30DH/Farm/BP_Tree.BP_Tree_C"))
            (for _array_element_2 _outactors_2
              (`/Engine/EditorBlueprintResources/StandardMacros.IsValid` (`/Game/30DH/Farm/BP_Tree.TreeCountdown` _array_element_2)
                (:`Is Valid`
                  (bind _treecountdown (`/Game/30DH/Farm/BP_Tree.TreeCountdown` _array_element_2))
                  (`/Game/30DH/Environment/BP_TreeCountdown.PollutionStart` _treecountdown (`/Game/30DH/Farm/BP_Tree.PollutionEffect` _array_element_2))
                  (`/Game/30DH/Environment/BP_TreeCountdown.TempStart` _treecountdown (`/Game/30DH/Farm/BP_Tree.TemperatureEffect` _array_element_2))
                  (`/Game/30DH/Environment/BP_TreeCountdown.HumidityStart` _treecountdown (`/Game/30DH/Farm/BP_Tree.HumidityEffect` _array_element_2)))))))))
    (:`then_1`
      (if (not (`/Game/30DH/Character/BP_Char.TimeOut` _returnvalue))
        ;[1 1 1] start check trigger for animal event
        (bind _returnvalue_5 (`GameplayStatics.GetActorOfClass` "/Game/30DH/Event/AnimalEvent/BP_AnimalTrigger.BP_AnimalTrigger_C"))
        (`/Game/30DH/Event/AnimalEvent/BP_AnimalTrigger.StartAnimalTrigger` _returnvalue_5)))))

(fn `UserConstructionScript`)