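; BP_LevelSelectItem is a level select item from the Modern Flat GUI Pack that holds enabled and selected state.
; Each setter stores its flag, then calls the OnSetEnabled or OnSetSelected dispatcher with the item and new value, so listeners can react.
; Two getters expose the current flags, and the file contains no visual or level-loading logic.
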(fn `IsEnabled`
  (returns (Enabled :type Boolean))
  (return (`self.bIsEnabled`)))

(fn `IsSelected`
  (returns (Selected :type Boolean))
  (return (`self.bIsSelected`)))

(fn `SetEnabled`
  (params (Enabled :type Boolean))
  (set `self.bIsEnabled` Enabled)
  (`self.OnSetEnabled` self (`self.bIsEnabled`)))

(fn `SetSelected`
  (params (Selected :type Boolean))
  (set `self.bIsSelected` Selected)
  (`self.OnSetSelected` self (`self.bIsSelected`)))