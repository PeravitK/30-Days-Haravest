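; BP_Timecontroller runs the day timer, driving the countdown widget, sun movement and timed river events.
; A looping one-second timer increments Second, updates the progress bar and pitches the DirectionalLight.
; Each tick checks the River actor's schedule to spawn fish and trash.
; At MaxSecond it stops the timer, flags BP_Char as timed out with its Sleepy visual and halts animal generation, while ResetTime restores the starting state.
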(event `self.ReceiveBeginPlay`
  (bind _returnvalue (`|CreateWidget` "/Game/30DH/Environment/Widget/WB_CountdownTime.WB_CountdownTime_C" (`GameplayStatics.GetPlayerController` 0)))
  (bind _output_get (set `self.WB_CountDownTime` _returnvalue))
  (`UserWidget.AddToViewport` _output_get 0)
  (`self.ResetTime`))

(event `StartTimer`
  (bind _returnvalue (`KismetSystemLibrary.K2_SetTimerDelegate` (delegate `Time++`) 1.0 true))
  (set `self.TimerHandle` _returnvalue))

(event `Time++`
  (bind _result (`/Engine/EditorBlueprintResources/StandardMacros.IncrementInt` (`self.Second`))
    (:`  `
      (bind _output_get (set `self.Second` _result))
      (set `self.DiractionalRotation` (+ 0.55 (`self.DiractionalRotation`)))
      (bind _returnvalue (`GameplayStatics.GetActorOfClass` "/Script/Engine.DirectionalLight"))
      (`self.K2_SetActorRotation` _returnvalue (`KismetMathLibrary.MakeRotator` 0.0 (`self.DiractionalRotation`)) false)
      (`/Game/30DH/Environment/Widget/WB_CountdownTime.SetPercent` (`self.WB_CountDownTime`) (/ (`KismetMathLibrary.Conv_IntToDouble` _output_get) (`self.MaxSecond`)))
      ;[1 1 1] spawn fish on random time
      (bind _returnvalue_2 (`GameplayStatics.GetActorOfClass` "/Game/30DH/Event/RiverEvent/River.River_C"))
      (if (== (`/Game/30DH/Event/RiverEvent/River.RandomTimeForFish` _returnvalue_2) (`self.Second`))
        (`/Game/30DH/Event/RiverEvent/River.SpawnFish` _returnvalue_2)
        (`/Game/30DH/Event/RiverEvent/River.TranslateFish` _returnvalue_2))
      (bind _returnvalue_3 (`GameplayStatics.GetActorOfClass` "/Game/30DH/Event/RiverEvent/River.River_C"))
      (bind _currentspawntrash (`/Game/30DH/Event/RiverEvent/River.CurrentSpawnTrash` _returnvalue_3))
      (bind _trashattr (`/Game/30DH/Event/RiverEvent/River.TrashAttr` _returnvalue_3))
      (if (>= _currentspawntrash (`KismetArrayLibrary.Array_Length` _trashattr))
        (if (>= _output_get (`self.MaxSecond`)) :!label _label
          (`self.TimerFinish`)
          (bind _returnvalue_4 (`GameplayStatics.GetActorOfClass` "/Game/30DH/Character/BP_Char.BP_Char_C"))
          (set `/Game/30DH/Character/BP_Char.TimeOut` true _returnvalue_4)
          (`SceneComponent.SetVisibility` (`/Game/30DH/Character/BP_Char.Sleepy` _returnvalue_4) true false)
          (bind _returnvalue_5 (`GameplayStatics.GetActorOfClass` "/Game/30DH/Event/AnimalEvent/BP_AnimalTrigger.BP_AnimalTrigger_C"))
          (`/Game/30DH/Event/AnimalEvent/BP_AnimalTrigger.StopGenerateAnimalEvent` _returnvalue_5))
        (elif (== (`self.Second`) (`.Time_5_574422324122B910EC27158AE7CFCE61` (break `/Game/30DH/Event/RiverEvent/TrashAttr` (`|GetArrayItem` _trashattr _currentspawntrash))))
          (`/Game/30DH/Event/RiverEvent/River.SpawnTrash` _returnvalue_3)
          (goto _label))))))

(event `TimerFinish`
  (`KismetSystemLibrary.K2_ClearAndInvalidateTimerHandle` (`self.TimerHandle`)))

(event `ResetTime`
  (`KismetSystemLibrary.K2_ClearAndInvalidateTimerHandle` (`self.TimerHandle`))
  (bind _output_get (set `self.Second` 0))
  (`/Engine/EditorBlueprintResources/StandardMacros.IsValid` (`self.WB_CountDownTime`)
    (:`Is Valid`
      (`/Game/30DH/Environment/Widget/WB_CountdownTime.SetPercent` (`self.WB_CountDownTime`) (`KismetMathLibrary.Conv_IntToDouble` _output_get))
      (bind _returnvalue (`GameplayStatics.GetActorOfClass` "/Script/Engine.DirectionalLight"))
      (`self.K2_SetActorRotation` _returnvalue (`KismetMathLibrary.MakeRotator` 0.0 190.0) false)
      (set `self.DiractionalRotation` 190.0))))

(fn `UserConstructionScript`)