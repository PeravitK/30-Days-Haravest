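; BP_Bed is the home bed that ends each day and triggers the end of the game on day 30.
; Collision overlaps register it in BP_Char's interactable list and refresh the outline.
; InteractBed toggles between Sleep, showing the day conclusion with movement disabled, and Wakeup.
; Wakeup either resets the game instance and shows the end screen, or briefly shows the day screen, restores movement and advances BP_EnvironmentSystem's day.
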(event `self.ReceiveActorBeginOverlap`
  (params (OtherActor :type "Actor Object Reference")))

(event `self.collision.OnComponentBeginOverlap`
  (params (OverlappedComponent :type "PrimitiveComponent Object Reference") (OtherActor :type "Actor Object Reference") (OtherComp :type "PrimitiveComponent Object Reference") (OtherBodyIndex :type Integer) (bFromSweep :type Boolean) (SweepResult :type "HitResult Structure (by ref)"))
  ;[1 1 1] add beginoverlap actor to currentoverlap&overlaparray
  (bind _asbp_char (cast `/Game/30DH/Character/BP_Char` OtherActor))
  (set `/Game/30DH/Character/BP_Char.CurrentOverlapObj` self _asbp_char)
  (`KismetArrayLibrary.Array_AddUnique` (`/Game/30DH/Character/BP_Char.OverlapObjArray` _asbp_char) self)
  (`/Game/30DH/Character/BP_Char.DisplayObjOutline` _asbp_char))

(event `self.collision.OnComponentEndOverlap`
  (params (OverlappedComponent :type "PrimitiveComponent Object Reference") (OtherActor :type "Actor Object Reference") (OtherComp :type "PrimitiveComponent Object Reference") (OtherBodyIndex :type Integer))
  (bind _asbp_char (cast `/Game/30DH/Character/BP_Char` OtherActor))
  (bind _overlapobjarray (`/Game/30DH/Character/BP_Char.OverlapObjArray` _asbp_char))
  (`KismetArrayLibrary.Array_Remove` _overlapobjarray (`KismetArrayLibrary.Array_Find` _overlapobjarray self))
  (if (== (`/Game/30DH/Character/BP_Char.CurrentOverlapObj` _asbp_char) self)
    ;[1 1 1] Check still have overlap in overlaparray?
    (if (`KismetArrayLibrary.Array_IsEmpty` _overlapobjarray)
      ;[1 1 1] if array empty -> currentoverlap = empty too
      (set `/Game/30DH/Character/BP_Char.CurrentOverlapObj` null _asbp_char)
      (else
        ;[1 1 1] if array not empty -> set currentoverlap = last obj in array
        (set `/Game/30DH/Character/BP_Char.CurrentOverlapObj` (`|GetArrayItem` _overlapobjarray (`KismetArrayLibrary.Array_LastIndex` _overlapobjarray)) _asbp_char)))
    (`/Game/30DH/Character/BP_Char.DisplayObjOutline` _asbp_char)))

(event `DisplayDayScreen`
  (bind _returnvalue (`GameplayStatics.GetPlayerController` 0))
  (bind _returnvalue_2 (`GameplayStatics.GetActorOfClass` "/Game/30DH/Character/BP_Char.BP_Char_C"))
  (`self.DisableInput` _returnvalue_2 _returnvalue)
  (bind _returnvalue_3 (`|CreateWidget` "/Game/30DH/Home/Widget/DayScreen.DayScreen_C" _returnvalue))
  (bind _output_get (set `self.WB_DayScreen` _returnvalue_3))
  (`UserWidget.AddToViewport` _output_get 10)
  (`KismetSystemLibrary.Delay` 2.0)
  (`Widget.RemoveFromParent` (`self.WB_DayScreen`))
  (set `self.WB_DayScreen` null)
  (`self.EnableInput` _returnvalue_2 _returnvalue))

(fn `InteractBed`
  (if (`self.ConclusionDisplay`)
    (`self.Wakeup`)
    (else
      (`self.Sleep`))))

(fn `Sleep`
  (`/Engine/EditorBlueprintResources/StandardMacros.IsValid` (`self.WB_DayScreen`)
    (:`Is Not Valid`
      (bind _returnvalue (`|CreateWidget` "/Game/30DH/Home/Widget/DayConclusion.DayConclusion_C" (`GameplayStatics.GetPlayerController` 0)))
      (bind _output_get (set `self.WB_DayConclusion` _returnvalue))
      (`UserWidget.AddToViewport` _output_get 10)
      (set `self.ConclusionDisplay` true)
      (bind _returnvalue_2 (`GameplayStatics.GetActorOfClass` "/Game/30DH/Character/BP_Char.BP_Char_C"))
      (`CharacterMovementComponent.DisableMovement` (`Character.CharacterMovement` _returnvalue_2)))))

(fn `UserConstructionScript`)

(fn `Wakeup`
  (bind _returnvalue (`GameplayStatics.GetPlayerController` 0))
  (`Widget.RemoveFromParent` (`self.WB_DayConclusion`))
  (bind _returnvalue_2 (`GameplayStatics.GetActorOfClass` "/Game/30DH/Environment/BP_EnvironmentSystem.BP_EnvironmentSystem_C"))
  (if (>= (`/Game/30DH/Environment/BP_EnvironmentSystem.Day` _returnvalue_2) 30)
    ;[1 1 1] EndGame
    (bind _asbp_30dh_instance (cast `/Game/30DH/Savegame/BP_30DH_Instance` (`GameplayStatics.GetGameInstance`)))
    (`/Game/30DH/Savegame/BP_30DH_Instance.Reset` _asbp_30dh_instance)
    (bind _returnvalue_3 (`|CreateWidget` "/Game/30DH/Start_End_UI/End_Screen.End_Screen_C"))
    (`UserWidget.AddToViewport` _returnvalue_3 1)
    (set `PlayerController.bShowMouseCursor` true _returnvalue)
    (`WidgetBlueprintLibrary.SetInputMode_UIOnlyEx` _returnvalue null)
    (else
      (`self.DisplayDayScreen`)
      (bind _returnvalue_4 (`GameplayStatics.GetActorOfClass` "/Game/30DH/Character/BP_Char.BP_Char_C"))
      (`CharacterMovementComponent.SetMovementMode` (`Character.CharacterMovement` _returnvalue_4) "MOVE_Walking" 0)
      (set `self.ConclusionDisplay` false)
      (bind _returnvalue_5 (`GameplayStatics.GetActorOfClass` "/Game/30DH/Environment/BP_EnvironmentSystem.BP_EnvironmentSystem_C"))
      (`/Game/30DH/Environment/BP_EnvironmentSystem.UpdateDay` _returnvalue_5))))