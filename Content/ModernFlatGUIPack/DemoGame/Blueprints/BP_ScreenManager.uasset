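; Screen manager for the farm demo game that creates and switches between the Title, Level Select and Level Complete UI screens.
; On BeginPlay it shows the cursor, adds all screens and the menu buttons to the viewport, then displays Title by toggling visibility.
; Bound button events switch screens, quit, open About, or start and reset levels through the farm game mode.
; Title visibility toggles the Home and Settings buttons, and number keys 1-5 are debug shortcuts.
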(event `self.ReceiveBeginPlay`
  (`self.Initialize`)
  (`self.ShowScreen` "NewEnumerator1"))

(event `Initialize`
  (`|ExecutionSequence`
    (:`then_0`
      (bind _output_get (set `self.PlayerController` (`GameplayStatics.GetPlayerController` 0)))
      (set `PlayerController.bShowMouseCursor` true _output_get))
    (:`then_1`
      (`self.InitTitleScreen`)
      (`self.InitLevelCompleteScreen`)
      (`self.InitLevelSelectScreen`)
      (`self.InitMenuButtons`))
    (:`then_2`
      (`self.HideAllScreens`))))

(event `ShowScreen`
  (params (Screen :type "/Game/ModernFlatGUIPack/Blueprints/E_ScreenType Enum" :default "NewEnumerator0"))
  (`self.HideAllScreens`)
  (switch `/Game/ModernFlatGUIPack/Blueprints/E_ScreenType` Screen
    (:`NewEnumerator1`
      (`Widget.SetVisibility` (`self.TitleScreen`) "Visible"))
    (:`NewEnumerator2`
      (`Widget.SetVisibility` (`self.LevelSelectScreen`) "Visible"))
    (:`NewEnumerator3`
      (`Widget.SetVisibility` (`self.LevelCompleteScreen`) "Visible"))))

(event `HideAllScreens`
  (`Widget.SetVisibility` (`self.TitleScreen`) "Hidden")
  (`Widget.SetVisibility` (`self.LevelSelectScreen`) "Hidden")
  (`Widget.SetVisibility` (`self.LevelCompleteScreen`) "Hidden"))

(event `InitTitleScreen`
  (bind _returnvalue (`|CreateWidget` "/Game/ModernFlatGUIPack/Widgets/WBP_TitleScreen.WBP_TitleScreen_C" (`self.PlayerController`)))
  (bind _output_get (set `self.TitleScreen` _returnvalue))
  (`UserWidget.AddToViewport` _output_get 0)
  (add `/Game/ModernFlatGUIPack/Widgets/WBP_TitleScreen.OnBtnPlayClicked` _output_get (`|CreateDelegate` :!event `OnTitleScreenBtnPlayClicked`))
  (add `/Game/ModernFlatGUIPack/Widgets/WBP_TitleScreen.OnBtnExitClicked` _output_get (`|CreateDelegate` :!event `OnTitleScreenBtnExitClicked`))
  (add `UserWidget.OnVisibilityChanged` _output_get (`|CreateDelegate` :!event `OnTitleScreenVisibilityChanged`)))

(event `OnTitleScreenBtnPlayClicked`
  (`self.ShowScreen` "NewEnumerator2")
  (`/Game/ModernFlatGUIPack/Widgets/WBP_LevelSelectScreen.SelectNextLevel` (`self.LevelSelectScreen`)))

(event `OnTitleScreenBtnExitClicked`
  (`KismetSystemLibrary.QuitGame` null "Quit"))

(event `OnTitleScreenVisibilityChanged`
  (params (InVisibility :type "ESlateVisibility Enum" :default "Visible"))
  (bind _btnhome (`/Game/ModernFlatGUIPack/Widgets/WBP_MenuButtons.BtnHome` (`self.MenuButtons`)))
  (bind _btnsettings (`/Game/ModernFlatGUIPack/Widgets/WBP_MenuButtons.BtnSettings` (`self.MenuButtons`)))
  (switch `ESlateVisibility` InVisibility
    (:`Visible`
      (`Widget.SetVisibility` _btnhome "Hidden")
      (`Widget.SetVisibility` _btnsettings "Hidden"))
    (:`Hidden`
      (`Widget.SetVisibility` _btnhome "Visible")
      (`Widget.SetVisibility` _btnsettings "Visible"))))

(event `InitLevelCompleteScreen`
  (bind _returnvalue (`|CreateWidget` "/Game/ModernFlatGUIPack/Widgets/WBP_LevelCompleteScreen.WBP_LevelCompleteScreen_C" (`self.PlayerController`)))
  (bind _output_get (set `self.LevelCompleteScreen` _returnvalue))
  (`UserWidget.AddToViewport` _output_get 0)
  (add `/Game/ModernFlatGUIPack/Widgets/WBP_LevelCompleteScreen.OnBtnReplayClicked` _output_get (`|CreateDelegate` :!event `OnLevelCompleteScreenBtnReplayClicked`))
  (add `/Game/ModernFlatGUIPack/Widgets/WBP_LevelCompleteScreen.OnBtnNextClicked` _output_get (`|CreateDelegate` :!event `OnLevelCompleteScreenBtnNextClicked`)))

(event `OnLevelCompleteScreenBtnNextClicked`
  (`self.ShowScreen` "NewEnumerator2")
  (`/Game/ModernFlatGUIPack/Widgets/WBP_LevelSelectScreen.SelectNextLevel` (`self.LevelSelectScreen`)))

(event `OnLevelCompleteScreenBtnReplayClicked`
  (`/Game/ModernFlatGUIPack/DemoGame/Blueprints/GM_FarmGame.StartLevel` (`/Game/ModernFlatGUIPack/DemoGame/Blueprints/BPFL_Demo.GetFarmGameMode`) (`/Game/ModernFlatGUIPack/DemoGame/Blueprints/GM_FarmGame.CurrentLevel` (`/Game/ModernFlatGUIPack/DemoGame/Blueprints/BPFL_Demo.GetFarmGameMode`)))
  (`self.ShowScreen` "NewEnumerator0"))

(event `InitLevelSelectScreen`
  (bind _returnvalue (`|CreateWidget` "/Game/ModernFlatGUIPack/Widgets/WBP_LevelSelectScreen.WBP_LevelSelectScreen_C" (`self.PlayerController`) (`/Game/ModernFlatGUIPack/DemoGame/Blueprints/GM_FarmGame.NumLevels` (`/Game/ModernFlatGUIPack/DemoGame/Blueprints/BPFL_Demo.GetFarmGameMode`))))
  (bind _output_get (set `self.LevelSelectScreen` _returnvalue))
  (`UserWidget.AddToViewport` _output_get 0)
  (add `/Game/ModernFlatGUIPack/Widgets/WBP_LevelSelectScreen.OnBtnPlayClicked` _output_get (`|CreateDelegate` :!event `OnLevelSelectScreenBtnPlayClicked`)))

(event `OnLevelSelectScreenBtnPlayClicked`
  (`/Game/ModernFlatGUIPack/DemoGame/Blueprints/GM_FarmGame.StartLevel` (`/Game/ModernFlatGUIPack/DemoGame/Blueprints/BPFL_Demo.GetFarmGameMode`) (`/Game/ModernFlatGUIPack/Widgets/WBP_LevelSelectScreen.GetSelectedLevel` (`self.LevelSelectScreen`)))
  (`self.ShowScreen` "NewEnumerator0"))

(event `InitMenuButtons`
  (bind _returnvalue (`|CreateWidget` "/Game/ModernFlatGUIPack/Widgets/WBP_MenuButtons.WBP_MenuButtons_C" (`self.PlayerController`)))
  (bind _output_get (set `self.MenuButtons` _returnvalue))
  (`UserWidget.AddToViewport` _output_get 0)
  (add `/Game/ModernFlatGUIPack/Widgets/WBP_MenuButtons.OnBtnHomeClicked` _output_get (`|CreateDelegate` :!event `OnMenuButtonsHomeBtnClicked`))
  (add `/Game/ModernFlatGUIPack/Widgets/WBP_MenuButtons.OnBtnAboutClicked` _output_get (`|CreateDelegate` :!event `OnMenuButtonsBtnAboutClicked`)))

(event `OnMenuButtonsHomeBtnClicked`
  (`/Game/ModernFlatGUIPack/DemoGame/Blueprints/GM_FarmGame.ResetGame` (`/Game/ModernFlatGUIPack/DemoGame/Blueprints/BPFL_Demo.GetFarmGameMode`))
  (`self.ShowScreen` "NewEnumerator1"))

(event `OnMenuButtonsBtnAboutClicked`
  (bind _returnvalue (`|CreateWidget` "/Game/ModernFlatGUIPack/Widgets/WBP_AboutScreen.WBP_AboutScreen_C" (`self.PlayerController`)))
  (`UserWidget.AddToViewport` _returnvalue 0))

(event `Key|One`
  (params (Key :type "Key Structure"))
  (:`Pressed`
    (`self.ShowScreen` "NewEnumerator0")))

(event `Key|Two`
  (params (Key :type "Key Structure"))
  (:`Pressed`
    (`self.ShowScreen` "NewEnumerator1")))

(event `Key|Three`
  (params (Key :type "Key Structure"))
  (:`Pressed`
    (`self.ShowScreen` "NewEnumerator2")))

(event `Key|Four`
  (params (Key :type "Key Structure"))
  (:`Pressed`
    (`self.ShowScreen` "NewEnumerator3")))

(event `Key|Five`
  (params (Key :type "Key Structure"))
  (:`Pressed`
    (bind _returnvalue (`|CreateWidget` "/Game/ModernFlatGUIPack/Widgets/WBP_AboutScreen.WBP_AboutScreen_C" (`self.PlayerController`)))
    (`UserWidget.AddToViewport` _returnvalue 0)))

(fn `UserConstructionScript`)