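; Blueprint function library for the Modern Flat GUI Pack that builds and adjusts button styles.
; GetButtonStyle looks up Normal, Hovered, Pressed and Disabled rows in ButtonTextureMap by composed key, returning texture-sized brushes and font styles, or printing on a missing row.
; Its optional size suffix always resolves to "_S" because the ButtonSize input is unused.
; ResetButtonTint sets all four state tints to white, preserving other style settings.
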(fn `GetButtonStyle`
  (params (Key :type String) (UseButtonSize :type Boolean) (ButtonSize :type "/Game/ModernFlatGUIPack/Blueprints/E_ButtonSize Enum" :default "NewEnumerator0"))
  (returns (BtnStyle :type "ButtonStyle Structure") (FontStyle :type "/Game/ModernFlatGUIPack/Blueprints/S_ButtonFontStyle Structure"))
  (locals (ButtonTextureMap :type "DataTable Object Reference" :default "DataTable'/Game/ModernFlatGUIPack/Data/DT_ButtonStyleMap.DT_ButtonStyleMap'") (TextureKey :type String))
  (set `local.TextureKey` Key)
  (if (`local.UseButtonSize`)
    (switch `/Game/ModernFlatGUIPack/Blueprints/E_ButtonSize` "NewEnumerator0"
      (:`NewEnumerator0`
        (set `local.TextureKey` (`KismetStringLibrary.Concat_StrStr` (`local.TextureKey`) "_S")))
      (:`NewEnumerator1`
        (set `local.TextureKey` (`KismetStringLibrary.Concat_StrStr` (`local.TextureKey`) "_M")))
      (:`NewEnumerator2`
        (set `local.TextureKey` (`KismetStringLibrary.Concat_StrStr` (`local.TextureKey`) "_L")))))
  (bind _returnvalue (`|GetDataTableRow` (`local.ButtonTextureMap`) (`KismetStringLibrary.Conv_StringToName` (`KismetStringLibrary.Concat_StrStr` (`local.TextureKey`) "_Normal")))
    (:`then`
      (bind _returnvalue_2 (`|GetDataTableRow` (`local.ButtonTextureMap`) (`KismetStringLibrary.Conv_StringToName` (`KismetStringLibrary.Concat_StrStr` (`local.TextureKey`) "_Hovered")))
        (:`then`
          (bind _returnvalue_3 (`|GetDataTableRow` (`local.ButtonTextureMap`) (`KismetStringLibrary.Conv_StringToName` (`KismetStringLibrary.Concat_StrStr` (`local.TextureKey`) "_Pressed")))
            (:`then`
              (bind _returnvalue_4 (`|GetDataTableRow` (`local.ButtonTextureMap`) (`KismetStringLibrary.Conv_StringToName` (`KismetStringLibrary.Concat_StrStr` (`local.TextureKey`) "_Disabled")))
                (:`then`
                  (bind (_texture _fontstyle) (break `/Game/ModernFlatGUIPack/Blueprints/S_ButtonStyleMap` _returnvalue))
                  (bind (_texture_2 _fontstyle_2) (break `/Game/ModernFlatGUIPack/Blueprints/S_ButtonStyleMap` _returnvalue_2))
                  (bind (_texture_3 _fontstyle_3) (break `/Game/ModernFlatGUIPack/Blueprints/S_ButtonStyleMap` _returnvalue_3))
                  (bind (_texture_4 _fontstyle_4) (break `/Game/ModernFlatGUIPack/Blueprints/S_ButtonStyleMap` _returnvalue_4))
                  (return (make `ButtonStyle` (make `SlateBrush` (`self.GetTextureSize` _texture (`local.__WorldContext`)) (struct) (struct :`SpecifiedColor` (struct :`R` 1.0 :`G` 1.0 :`B` 1.0 :`A` 1.0) :`ColorUseRule` "UseColor_Specified") _texture) (make `SlateBrush` (`self.GetTextureSize` _texture_2 (`local.__WorldContext`)) (struct) (struct :`SpecifiedColor` (struct :`R` 1.0 :`G` 1.0 :`B` 1.0 :`A` 1.0) :`ColorUseRule` "UseColor_Specified") _texture_2) (make `SlateBrush` (`self.GetTextureSize` _texture_3 (`local.__WorldContext`)) (struct) (struct :`SpecifiedColor` (struct :`R` 1.0 :`G` 1.0 :`B` 1.0 :`A` 1.0) :`ColorUseRule` "UseColor_Specified") _texture_3) (make `SlateBrush` (`self.GetTextureSize` _texture_4 (`local.__WorldContext`)) (struct) (struct :`SpecifiedColor` (struct :`R` 1.0 :`G` 1.0 :`B` 1.0 :`A` 1.0) :`ColorUseRule` "UseColor_Specified") _texture_4)) (make `/Game/ModernFlatGUIPack/Blueprints/S_ButtonFontStyle` _fontstyle _fontstyle_2 _fontstyle_3 _fontstyle_4)))
                (:`RowNotFound`
                  _)))
            (:`RowNotFound`
              _)))
        (:`RowNotFound`
          _)))
    (:`RowNotFound`
      _))
  (`KismetSystemLibrary.PrintString` (`local.__WorldContext`) "Button Style Not Found")
  (return))

(fn `GetTextureSize`
  (params (InTexture :type "Texture2D Object Reference"))
  (returns (OutSize :type "Vector2D Structure"))
  (return (`KismetMathLibrary.MakeVector2D` (`KismetMathLibrary.Conv_IntToDouble` (`Texture2D.Blueprint_GetSizeX` InTexture)) (`KismetMathLibrary.Conv_IntToDouble` (`Texture2D.Blueprint_GetSizeY` InTexture)))))

(fn `ResetButtonTint`
  (params (Button :type "Button Object Reference"))
  (locals (CurrStyle :type "ButtonStyle Structure"))
  (bind _slatecolor (make `SlateColor` (struct :`R` 1.0 :`G` 1.0 :`B` 1.0 :`A` 1.0)))
  (bind _widgetstyle (`Button.WidgetStyle` Button))
  (`Button.SetStyle` Button (make `ButtonStyle` (make `SlateBrush` (break `SlateBrush` (break `ButtonStyle` _widgetstyle)) (`.Margin` (break `SlateBrush` (break `ButtonStyle` _widgetstyle))) _slatecolor (`.ResourceObject` (break `SlateBrush` (break `ButtonStyle` _widgetstyle))) (`.DrawAs` (break `SlateBrush` (break `ButtonStyle` _widgetstyle))) (`.Tiling` (break `SlateBrush` (break `ButtonStyle` _widgetstyle))) (`.Mirroring` (break `SlateBrush` (break `ButtonStyle` _widgetstyle)))) (make `SlateBrush` (break `SlateBrush` (`.Hovered` (break `ButtonStyle` _widgetstyle))) (`.Margin` (break `SlateBrush` (`.Hovered` (break `ButtonStyle` _widgetstyle)))) _slatecolor (`.ResourceObject` (break `SlateBrush` (`.Hovered` (break `ButtonStyle` _widgetstyle)))) (`.DrawAs` (break `SlateBrush` (`.Hovered` (break `ButtonStyle` _widgetstyle)))) (`.Tiling` (break `SlateBrush` (`.Hovered` (break `ButtonStyle` _widgetstyle)))) (`.Mirroring` (break `SlateBrush` (`.Hovered` (break `ButtonStyle` _widgetstyle))))) (make `SlateBrush` (break `SlateBrush` (`.Pressed` (break `ButtonStyle` _widgetstyle))) (`.Margin` (break `SlateBrush` (`.Pressed` (break `ButtonStyle` _widgetstyle)))) _slatecolor (`.ResourceObject` (break `SlateBrush` (`.Pressed` (break `ButtonStyle` _widgetstyle)))) (`.DrawAs` (break `SlateBrush` (`.Pressed` (break `ButtonStyle` _widgetstyle)))) (`.Tiling` (break `SlateBrush` (`.Pressed` (break `ButtonStyle` _widgetstyle)))) (`.Mirroring` (break `SlateBrush` (`.Pressed` (break `ButtonStyle` _widgetstyle))))) (make `SlateBrush` (break `SlateBrush` (`.Disabled` (break `ButtonStyle` _widgetstyle))) (`.Margin` (break `SlateBrush` (`.Disabled` (break `ButtonStyle` _widgetstyle)))) _slatecolor (`.ResourceObject` (break `SlateBrush` (`.Disabled` (break `ButtonStyle` _widgetstyle)))) (`.DrawAs` (break `SlateBrush` (`.Disabled` (break `ButtonStyle` _widgetstyle)))) (`.Tiling` (break `SlateBrush` (`.Disabled` (break `ButtonStyle` _widgetstyle)))) (`.Mirroring` (break `SlateBrush` (`.Disabled` (break `ButtonStyle` _widgetstyle))))) (`.NormalPadding` (break `ButtonStyle` _widgetstyle)) (`.PressedPadding` (break `ButtonStyle` _widgetstyle)) (`.PressedSlateSound` (break `ButtonStyle` _widgetstyle)) (`.HoveredSlateSound` (break `ButtonStyle` _widgetstyle)))))