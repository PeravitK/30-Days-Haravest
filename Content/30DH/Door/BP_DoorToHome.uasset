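; BP_DoorToHome is a door that moves the player character to the Home location.
; Its collision overlaps register or remove the door in BP_Char's overlap list, update the current overlap object and refresh the outline display.
; GoToHome updates the character's location and widget, teleports it to a hardcoded transform, and switches view to the camera found by display name "Home_CameraActor".
; It also tells BP_AnimalTrigger to stop generating animal events.
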(event `self.Collision.OnComponentBeginOverlap`
  (params (OverlappedComponent :type "PrimitiveComponent Object Reference") (OtherActor :type "Actor Object Reference") (OtherComp :type "PrimitiveComponent Object Reference") (OtherBodyIndex :type Integer) (bFromSweep :type Boolean) (SweepResult :type "HitResult Structure (by ref)"))
  ;[1 1 1] add beginoverlap actor to currentoverlap&overlaparray
  (bind _asbp_char (cast `/Game/30DH/Character/BP_Char` OtherActor))
  (set `/Game/30DH/Character/BP_Char.CurrentOverlapObj` self _asbp_char)
  (`KismetArrayLibrary.Array_AddUnique` (`/Game/30DH/Character/BP_Char.OverlapObjArray` _asbp_char) self)
  (`/Game/30DH/Character/BP_Char.DisplayObjOutline` _asbp_char))

(event `self.Collision.OnComponentEndOverlap`
  (params (OverlappedComponent :type "PrimitiveComponent Object Reference") (OtherActor :type "Actor Object Reference") (OtherComp :type "PrimitiveComponent Object Reference") (OtherBodyIndex :type Integer))
  (bind _asbp_char (cast `/Game/30DH/Character/BP_Char` OtherActor))
  (bind _overlapobjarray (`/Game/30DH/Character/BP_Char.OverlapObjArray` _asbp_char))
  (`KismetArrayLibrary.Array_Remove` _overlapobjarray (`KismetArrayLibrary.Array_Find` _overlapobjarray self))
  ;[1 1 1] Check Currentoverlap == endoverlaptrigger?
  (if (== (`/Game/30DH/Character/BP_Char.CurrentOverlapObj` _asbp_char) self)
    ;[1 1 1] Check still have overlap in overlaparray?
    (if (`KismetArrayLibrary.Array_IsEmpty` _overlapobjarray)
      ;[1 1 1] if array empty -> currentoverlap = empty too
      (set `/Game/30DH/Character/BP_Char.CurrentOverlapObj` null _asbp_char)
      (else
        ;[1 1 1] if array not empty -> set currentoverlap = last obj in array
        (set `/Game/30DH/Character/BP_Char.CurrentOverlapObj` (`|GetArrayItem` _overlapobjarray (`KismetArrayLibrary.Array_LastIndex` _overlapobjarray)) _asbp_char)))
    (`/Game/30DH/Character/BP_Char.DisplayObjOutline` _asbp_char)))

(fn `GoToHome`
  (`|ExecutionSequence`
    (:`then_0`
      (bind _returnvalue (`GameplayStatics.GetActorOfClass` "/Game/30DH/Character/BP_Char.BP_Char_C"))
      (`|ExecutionSequence`
        (:`then_0`
          ;[1 1 1] update widget
          (set `/Game/30DH/Character/BP_Char.CurrentLocation` "Home" _returnvalue)
          (`/Game/30DH/Character/BP_Char.ManageWidget` _returnvalue))
        (:`then_1`
          ;[1 1 1] set character location
          (bind _returnvalue_2 (`GameplayStatics.GetActorOfClass` "/Game/30DH/Character/BP_Char.BP_Char_C"))
          (`self.K2_SetActorLocationAndRotation` _returnvalue_2 (-100.0 -1720.0 90.0) (struct :`Yaw` -90.0) false false))
        (:`then_2`
          ;[1 1 1] set camera
          (bind _outactors (`GameplayStatics.GetAllActorsOfClass` "/Script/Engine.CameraActor"))
          (for _array_element _outactors
            (if (`KismetStringLibrary.EqualEqual_StrStr` (`KismetSystemLibrary.GetDisplayName` _array_element) "Home_CameraActor")
              (`PlayerController.SetViewTargetWithBlend` (`PlayerState.GetPlayerController` (`Pawn.PlayerState` _returnvalue)) _array_element 0.0 "VTBlend_Linear" 0.0 false))))))
    (:`then_1`
      ;[1 1 1] stop check trigger for animal event
      (bind _returnvalue_3 (`GameplayStatics.GetActorOfClass` "/Game/30DH/Event/AnimalEvent/BP_AnimalTrigger.BP_AnimalTrigger_C"))
      (`/Game/30DH/Event/AnimalEvent/BP_AnimalTrigger.StopGenerateAnimalEvent` _returnvalue_3))))

(fn `UserConstructionScript`)