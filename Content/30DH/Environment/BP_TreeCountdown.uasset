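; Countdown actor that gradually applies a tree's pollution, temperature and humidity effects to BP_EnvironmentSystem, or reverses them when the matching Cutting flag is set.
; Each Start event runs a looping one-second timer that shifts that value one point per tick and refreshes every BP_Crop's suitability display.
; Pollution only steps for negative amounts, while temperature and humidity handle both signs.
; Timers stop at their targets, and the actor destroys itself once all three finish and IsReset is set.
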(event `PollutionBreakLoop`
  (`KismetSystemLibrary.K2_ClearAndInvalidateTimerHandle` (`self.PollutionTimer`))
  (bind _output_get (set `self.EndPollution` true))
  (if (and _output_get (stale `TempBreakLoop` _output_get) (stale `HumidityBreakLoop` _output_get)) :!label _label
    (if (`self.IsReset`)
      (`self.K2_DestroyActor`))))

(event `TempBreakLoop`
  (`KismetSystemLibrary.K2_ClearAndInvalidateTimerHandle` (`self.TempTimer`))
  (bind _output_get (set `self.EndTemp` true))
  (goto _label))

(event `HumidityBreakLoop`
  (`KismetSystemLibrary.K2_ClearAndInvalidateTimerHandle` (`self.HumifdityTimer`))
  (bind _output_get (set `self.EndHumidity` true))
  (goto _label))

(event `PollutionStart`
  (params (PollutionFromTree :type Integer))
  (set `self.EndPollution` false)
  (bind _returnvalue (`KismetSystemLibrary.K2_SetTimerDelegate` (delegate `PollutionLoop`) 1.0 true))
  (set `self.PollutionTimer` _returnvalue))

(event `PollutionLoop`
  (if (`self.PollutionCutting`)
    (if (< (stale `PollutionStart` PollutionFromTree) 0)
      (if (== (* (`self.PollutionChecked`) -1) (stale `PollutionStart` PollutionFromTree))
        (set `self.PollutionChecked` 0)
        (set `self.PollutionCutting` false)
        (`self.PollutionBreakLoop`)
        (else
          (bind _returnvalue (`GameplayStatics.GetActorOfClass` "/Game/30DH/Environment/BP_EnvironmentSystem.BP_EnvironmentSystem_C"))
          (set `/Game/30DH/Environment/BP_EnvironmentSystem.TodayPollution` (+ (`/Game/30DH/Environment/BP_EnvironmentSystem.TodayPollution` _returnvalue) 1) _returnvalue)
          (set `self.PollutionChecked` (+ (`self.PollutionChecked`) 1))
          (bind _outactors (`GameplayStatics.GetAllActorsOfClass` "/Game/30DH/Farm/BP_Crop.BP_Crop_C"))
          (for _array_element _outactors
            (`/Game/30DH/Farm/BP_Crop.EnvironmentSuitableChecker&Display` _array_element)))))
    (elif (< (stale `PollutionStart` PollutionFromTree) 0)
      (if (== (stale `PollutionStart` PollutionFromTree) (`self.PollutionChecked`))
        (set `self.PollutionChecked` 0)
        (set `self.PollutionCutting` false)
        (`self.PollutionBreakLoop`)
        (else
          (bind _returnvalue_2 (`GameplayStatics.GetActorOfClass` "/Game/30DH/Environment/BP_EnvironmentSystem.BP_EnvironmentSystem_C"))
          (set `/Game/30DH/Environment/BP_EnvironmentSystem.TodayPollution` (- (`/Game/30DH/Environment/BP_EnvironmentSystem.TodayPollution` _returnvalue_2) 1) _returnvalue_2)
          (set `self.PollutionChecked` (- (`self.PollutionChecked`) 1))
          (bind _outactors_2 (`GameplayStatics.GetAllActorsOfClass` "/Game/30DH/Farm/BP_Crop.BP_Crop_C"))
          (for _array_element_2 _outactors_2
            (`/Game/30DH/Farm/BP_Crop.EnvironmentSuitableChecker&Display` _array_element_2)))))))

(event `TempStart`
  (params (TempFromTree :type Integer))
  (set `self.EndTemp` false)
  (bind _returnvalue (`KismetSystemLibrary.K2_SetTimerDelegate` (delegate `TempLoop`) 1.0 true))
  (set `self.TempTimer` _returnvalue))

(event `TempLoop`
  (if (`self.TempCutting`)
    (if (< (stale `TempStart` TempFromTree) 0)
      (if (== (* (`self.TempChecked`) -1) (stale `TempStart` TempFromTree))
        (set `self.TempChecked` 0)
        (set `self.TempCutting` false)
        (`self.TempBreakLoop`)
        (else
          (bind _returnvalue (`GameplayStatics.GetActorOfClass` "/Game/30DH/Environment/BP_EnvironmentSystem.BP_EnvironmentSystem_C"))
          (set `/Game/30DH/Environment/BP_EnvironmentSystem.TodayTemp` (+ (`/Game/30DH/Environment/BP_EnvironmentSystem.TodayTemp` _returnvalue) 1) _returnvalue)
          (set `self.TempChecked` (+ (`self.TempChecked`) 1))
          (bind _outactors (`GameplayStatics.GetAllActorsOfClass` "/Game/30DH/Farm/BP_Crop.BP_Crop_C"))
          (for _array_element _outactors
            (`/Game/30DH/Farm/BP_Crop.EnvironmentSuitableChecker&Display` _array_element))))
      (elif (== (* (`self.TempChecked`) -1) (stale `TempStart` TempFromTree))
        (set `self.TempChecked` 0)
        (set `self.TempCutting` false)
        (`self.TempBreakLoop`)
        (else
          (bind _returnvalue_2 (`GameplayStatics.GetActorOfClass` "/Game/30DH/Environment/BP_EnvironmentSystem.BP_EnvironmentSystem_C"))
          (set `/Game/30DH/Environment/BP_EnvironmentSystem.TodayTemp` (- (`/Game/30DH/Environment/BP_EnvironmentSystem.TodayTemp` _returnvalue_2) 1) _returnvalue_2)
          (set `self.TempChecked` (- (`self.TempChecked`) 1))
          (bind _outactors_2 (`GameplayStatics.GetAllActorsOfClass` "/Game/30DH/Farm/BP_Crop.BP_Crop_C"))
          (for _array_element_2 _outactors_2
            (`/Game/30DH/Farm/BP_Crop.EnvironmentSuitableChecker&Display` _array_element_2)))))
    (elif (< (stale `TempStart` TempFromTree) 0)
      (if (== (`self.TempChecked`) (stale `TempStart` TempFromTree))
        (set `self.TempChecked` 0)
        (set `self.PollutionCutting` false)
        (`self.TempBreakLoop`)
        (else
          (bind _returnvalue_3 (`GameplayStatics.GetActorOfClass` "/Game/30DH/Environment/BP_EnvironmentSystem.BP_EnvironmentSystem_C"))
          (set `/Game/30DH/Environment/BP_EnvironmentSystem.TodayTemp` (- (`/Game/30DH/Environment/BP_EnvironmentSystem.TodayTemp` _returnvalue_3) 1) _returnvalue_3)
          (set `self.TempChecked` (- (`self.TempChecked`) 1))
          (bind _outactors_3 (`GameplayStatics.GetAllActorsOfClass` "/Game/30DH/Farm/BP_Crop.BP_Crop_C"))
          (for _array_element_3 _outactors_3
            (`/Game/30DH/Farm/BP_Crop.EnvironmentSuitableChecker&Display` _array_element_3))))
      (elif (== (`self.TempChecked`) (stale `TempStart` TempFromTree))
        (set `self.TempChecked` 0)
        (set `self.PollutionCutting` false)
        (`self.TempBreakLoop`)
        (else
          (bind _returnvalue_4 (`GameplayStatics.GetActorOfClass` "/Game/30DH/Environment/BP_EnvironmentSystem.BP_EnvironmentSystem_C"))
          (set `/Game/30DH/Environment/BP_EnvironmentSystem.TodayTemp` (+ (`/Game/30DH/Environment/BP_EnvironmentSystem.TodayTemp` _returnvalue_4) 1) _returnvalue_4)
          (set `self.TempChecked` (+ (`self.TempChecked`) 1))
          (bind _outactors_4 (`GameplayStatics.GetAllActorsOfClass` "/Game/30DH/Farm/BP_Crop.BP_Crop_C"))
          (for _array_element_4 _outactors_4
            (`/Game/30DH/Farm/BP_Crop.EnvironmentSuitableChecker&Display` _array_element_4)))))))

(event `HumidityStart`
  (params (HumidityFromTree :type Integer))
  (set `self.EndHumidity` false)
  (bind _returnvalue (`KismetSystemLibrary.K2_SetTimerDelegate` (delegate `HumidityLoop`) 1.0 true))
  (set `self.HumifdityTimer` _returnvalue))

(event `HumidityLoop`
  (if (`self.HumidityCutting`)
    (if (< (stale `HumidityStart` HumidityFromTree) 0)
      (if (== (* (`self.HumidityChecked`) -1) (stale `HumidityStart` HumidityFromTree))
        (set `self.HumidityChecked` 0)
        (set `self.HumidityCutting` false)
        (`self.HumidityBreakLoop`)
        (else
          (bind _returnvalue (`GameplayStatics.GetActorOfClass` "/Game/30DH/Environment/BP_EnvironmentSystem.BP_EnvironmentSystem_C"))
          (set `/Game/30DH/Environment/BP_EnvironmentSystem.TodayHumidity` (+ (`/Game/30DH/Environment/BP_EnvironmentSystem.TodayHumidity` _returnvalue) 1) _returnvalue)
          (set `self.HumidityChecked` (+ (`self.HumidityChecked`) 1))
          (bind _outactors (`GameplayStatics.GetAllActorsOfClass` "/Game/30DH/Farm/BP_Crop.BP_Crop_C"))
          (for _array_element _outactors
            (`/Game/30DH/Farm/BP_Crop.EnvironmentSuitableChecker&Display` _array_element))))
      (elif (== (* (`self.HumidityChecked`) -1) (stale `HumidityStart` HumidityFromTree))
        (set `self.HumidityChecked` 0)
        (set `self.HumidityCutting` false)
        (`self.HumidityBreakLoop`)
        (else
          (bind _returnvalue_2 (`GameplayStatics.GetActorOfClass` "/Game/30DH/Environment/BP_EnvironmentSystem.BP_EnvironmentSystem_C"))
          (set `/Game/30DH/Environment/BP_EnvironmentSystem.TodayHumidity` (- (`/Game/30DH/Environment/BP_EnvironmentSystem.TodayHumidity` _returnvalue_2) 1) _returnvalue_2)
          (set `self.HumidityChecked` (- (`self.HumidityChecked`) 1))
          (bind _outactors_2 (`GameplayStatics.GetAllActorsOfClass` "/Game/30DH/Farm/BP_Crop.BP_Crop_C"))
          (for _array_element_2 _outactors_2
            (`/Game/30DH/Farm/BP_Crop.EnvironmentSuitableChecker&Display` _array_element_2)))))
    (elif (< (stale `HumidityStart` HumidityFromTree) 0)
      (if (== (`self.HumidityChecked`) (stale `HumidityStart` HumidityFromTree))
        (set `self.HumidityChecked` 0)
        (set `self.HumidityCutting` false)
        (`self.HumidityBreakLoop`)
        (else
          (bind _returnvalue_3 (`GameplayStatics.GetActorOfClass` "/Game/30DH/Environment/BP_EnvironmentSystem.BP_EnvironmentSystem_C"))
          (set `/Game/30DH/Environment/BP_EnvironmentSystem.TodayHumidity` (- (`/Game/30DH/Environment/BP_EnvironmentSystem.TodayHumidity` _returnvalue_3) 1) _returnvalue_3)
          (set `self.HumidityChecked` (- (`self.HumidityChecked`) 1))
          (bind _outactors_3 (`GameplayStatics.GetAllActorsOfClass` "/Game/30DH/Farm/BP_Crop.BP_Crop_C"))
          (for _array_element_3 _outactors_3
            (`/Game/30DH/Farm/BP_Crop.EnvironmentSuitableChecker&Display` _array_element_3))))
      (elif (== (`self.HumidityChecked`) (stale `HumidityStart` HumidityFromTree))
        (set `self.HumidityChecked` 0)
        (set `self.HumidityCutting` false)
        (`self.HumidityBreakLoop`)
        (else
          (bind _returnvalue_4 (`GameplayStatics.GetActorOfClass` "/Game/30DH/Environment/BP_EnvironmentSystem.BP_EnvironmentSystem_C"))
          (set `/Game/30DH/Environment/BP_EnvironmentSystem.TodayHumidity` (+ (`/Game/30DH/Environment/BP_EnvironmentSystem.TodayHumidity` _returnvalue_4) 1) _returnvalue_4)
          (set `self.HumidityChecked` (+ (`self.HumidityChecked`) 1))
          (bind _outactors_4 (`GameplayStatics.GetAllActorsOfClass` "/Game/30DH/Farm/BP_Crop.BP_Crop_C"))
          (for _array_element_4 _outactors_4
            (`/Game/30DH/Farm/BP_Crop.EnvironmentSuitableChecker&Display` _array_element_4)))))))

(fn `UserConstructionScript`)