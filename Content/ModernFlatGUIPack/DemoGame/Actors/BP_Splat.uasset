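; BP_Splat is a short-lived debris burst actor from the ModernFlatGUIPack demo game.
; On BeginPlay it gives its Scene a random yaw and collects the child static mesh components into ExplodableMeshes.
; It turns on physics for each mesh, then launches it with an upward velocity impulse plus a radial impulse from the Scene's location.
; Tick accumulates lifetime and destroys the actor once TotalLifetime is reached.
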(event `self.ReceiveBeginPlay`
  (`|ExecutionSequence`
    (:`then_0`
      (`SceneComponent.K2_SetWorldRotation` (`self.Scene`) (`KismetMathLibrary.MakeRotator` 0.0 0.0 (`KismetMathLibrary.RandomFloatInRange` 0.0 360.0)) false false))
    (:`then_1`
      (for _array_element (`SceneComponent.GetChildrenComponents` (`self.Scene`) true)
        (bind _asstatic_mesh_component (cast `StaticMeshComponent` _array_element))
        (`KismetArrayLibrary.Array_Add` (`self.ExplodableMeshes`) _asstatic_mesh_component)))
    (:`then_2`
      (for _array_element_2 (`self.ExplodableMeshes`)
        (`PrimitiveComponent.SetSimulatePhysics` _array_element_2 true)
        (`PrimitiveComponent.AddImpulse` _array_element_2 (0.0 0.0 200.0) "None" true)
        (`PrimitiveComponent.AddRadialImpulse` _array_element_2 (`SceneComponent.K2_GetComponentLocation` (`self.Scene`)) 50.0 10.0 "RIF_Constant" false)))))

(event `self.ReceiveTick`
  (params (DeltaSeconds :type "Float (single-precision)"))
  (set `self.CurrLifetime` (+ DeltaSeconds (`self.CurrLifetime`)))
  (if (>= (`self.CurrLifetime`) (`self.TotalLifetime`))
    (`self.K2_DestroyActor`)))

(fn `UserConstructionScript`)