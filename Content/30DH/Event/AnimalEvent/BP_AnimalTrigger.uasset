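; BP_AnimalTrigger randomly spawns duck and mole animal events on the farm, capped by a per-day event count.
; StartAnimalTrigger runs a one-second looping timer that recounts grown crops and tilled, unseeded plots until StopGenerateAnimalEvent clears it.
; Duck odds rise with grown crops, while mole odds fall as empty tilled plots increase, requiring at least one.
; Both spawn with BT_Animal at a random X along a fixed Y line.
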(event `self.ReceiveTick`
  (params (DeltaSeconds :type "Float (single-precision)")))

(event `StartAnimalTrigger`
  (bind _returnvalue (`KismetSystemLibrary.K2_SetTimerDelegate` (delegate `GenerateAnimalEvent`) 1.0 true))
  (set `self.AnimalTriggerTimer` _returnvalue))

(event `GenerateAnimalEvent`
  (`|ExecutionSequence`
    (:`then_0`
      ;[1 1 1] reset every loop
      (set `self.FullyGrownCrop` 0)
      (set `self.ReadyToSeedPlot` 0)
      (`|ExecutionSequence`
        (:`then_0`
          ;[1 1 1] count fully grown crop
          (bind _outactors (`GameplayStatics.GetAllActorsOfClass` "/Game/30DH/Farm/BP_Crop.BP_Crop_C"))
          (for _array_element _outactors
            (if (`/Game/30DH/Farm/BP_Crop.FullyGrownCheck` _array_element)
              (`/Engine/EditorBlueprintResources/StandardMacros.IncrementInt` (`self.FullyGrownCrop`)))))
        (:`then_1`
          ;[1 1 1] count ready to seed plot
          (bind _outactors_2 (`GameplayStatics.GetAllActorsOfClass` "/Game/30DH/Farm/BP_Plot.BP_Plot_C"))
          (for _array_element_2 _outactors_2
            (if (and (`/Game/30DH/Farm/BP_Plot.TillSoilCheck` _array_element_2) (not (`/Game/30DH/Farm/BP_Plot.SeedPlantCheck` _array_element_2)))
              (`/Engine/EditorBlueprintResources/StandardMacros.IncrementInt` (`self.ReadyToSeedPlot`)))))))
    (:`then_1`
      (`|ExecutionSequence`
        (:`then_0`
          (if (>= (`self.CountEventPerDay`) (`self.MaxEventPerDay`))
            _
            (elif (> (`self.FullyGrownCrop`) 0)
              (if (<= (`KismetMathLibrary.RandomFloatInRange` 1.0 100.0) (+ (`self.DuckSpawnRate`) (* (`self.FullyGrownCrop`) 0.5)))
                (`AIBlueprintHelperLibrary.SpawnAIFromClass` "/Game/30DH/Event/AnimalEvent/BP_Duck.BP_Duck_C" "/Game/30DH/Event/AnimalEvent/Duck_AI/BT_Animal.BT_Animal" (.location (`KismetMathLibrary.MakeTransform` (`KismetMathLibrary.MakeVector` (`KismetMathLibrary.RandomFloatInRange` -120.0 450.0) 850.0))) (.rotation (`KismetMathLibrary.MakeTransform` (`KismetMathLibrary.MakeVector` (`KismetMathLibrary.RandomFloatInRange` -120.0 450.0) 850.0))) false null)
                (`/Engine/EditorBlueprintResources/StandardMacros.IncrementInt` (`self.CountEventPerDay`))))))
        (:`then_1`
          (if (>= (`self.CountEventPerDay`) (`self.MaxEventPerDay`))
            _
            (elif (> (`self.ReadyToSeedPlot`) 0)
              (if (<= (`KismetMathLibrary.RandomFloatInRange` 1.0 100.0) (+ (`self.MoleSpawnRate`) (- 10.5 (* (- (`self.ReadyToSeedPlot`) 1) 0.5))))
                (`AIBlueprintHelperLibrary.SpawnAIFromClass` "/Game/30DH/Event/AnimalEvent/BP_Mole.BP_Mole_C" "/Game/30DH/Event/AnimalEvent/Duck_AI/BT_Animal.BT_Animal" (.location (`KismetMathLibrary.MakeTransform` (`KismetMathLibrary.MakeVector` (`KismetMathLibrary.RandomFloatInRange` -120.0 450.0) 850.0))) (.rotation (`KismetMathLibrary.MakeTransform` (`KismetMathLibrary.MakeVector` (`KismetMathLibrary.RandomFloatInRange` -120.0 450.0) 850.0))) false null)
                (`/Engine/EditorBlueprintResources/StandardMacros.IncrementInt` (`self.CountEventPerDay`))))))))))

(event `StopGenerateAnimalEvent`
  (`KismetSystemLibrary.K2_ClearAndInvalidateTimerHandle` (`self.AnimalTriggerTimer`)))

(fn `UserConstructionScript`)