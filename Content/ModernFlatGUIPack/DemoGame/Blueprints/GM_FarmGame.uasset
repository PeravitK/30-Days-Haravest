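; Game mode for the GUI pack's farm demo game, running levels built around clearing spawned dogs.
; StartLevel removes existing dogs and spawns twice the level number at random positions and yaws, calling SpawnDefaultController through each one's Instigator.
; DecrementDog counts down the remaining dogs and triggers CompleteLevel at zero.
; After a short delay, CompleteLevel switches screens through the screen manager, updates level select and shows a score based solely on level number.
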(event `StartLevel`
  (params (LevelNum :type Integer))
  (`self.ResetGame`)
  (set `self.Score` 0)
  (`self.SpawnDogs` (* LevelNum 2))
  (set `self.CurrentLevel` LevelNum))

(event `SpawnDogs`
  (params (NumDogs :type Integer))
  (set `self.DogsRemaining` NumDogs)
  (for _ (range 1 (+ NumDogs 1))
    (bind _returnvalue (`|SpawnActorFromClass` "/Game/ModernFlatGUIPack/DemoGame/Actors/BP_Dog.BP_Dog_C" (`KismetMathLibrary.MakeTransform` (`KismetMathLibrary.MakeVector` (`KismetMathLibrary.RandomFloatInRange` -300.0 300.0) (`KismetMathLibrary.RandomFloatInRange` -300.0 300.0) 34.0) (`KismetMathLibrary.MakeRotator` 0.0 0.0 (`KismetMathLibrary.RandomFloatInRange` 0.0 360.0))) "AdjustIfPossibleButAlwaysSpawn" "OverrideRootScale" null null))
    (`Pawn.SpawnDefaultController` (`Actor.Instigator` _returnvalue))))

(event `DecrementDog`
  (`/Engine/EditorBlueprintResources/StandardMacros.DecrementInt` (`self.DogsRemaining`)
    (:`  `
      (if (== (`self.DogsRemaining`) 0)
        (`self.CompleteLevel`)))))

(event `ResetGame`
  (bind _outactors (`GameplayStatics.GetAllActorsOfClass` "/Game/ModernFlatGUIPack/DemoGame/Actors/BP_Dog.BP_Dog_C"))
  (for _array_element _outactors
    (`self.K2_DestroyActor` _array_element))
  (set `self.DogsRemaining` 0))

(event `CompleteLevel`
  (`KismetSystemLibrary.Delay` 1.0)
  (`/Game/ModernFlatGUIPack/DemoGame/Blueprints/BP_ScreenManager.ShowScreen` (`/Game/ModernFlatGUIPack/DemoGame/Blueprints/BPFL_Demo.GetScreenManager`) "NewEnumerator3")
  (`/Game/ModernFlatGUIPack/Widgets/WBP_LevelSelectScreen.CompleteLevel` (`/Game/ModernFlatGUIPack/DemoGame/Blueprints/BP_ScreenManager.LevelSelectScreen` (`/Game/ModernFlatGUIPack/DemoGame/Blueprints/BPFL_Demo.GetScreenManager`)) (`self.CurrentLevel`))
  (`/Game/ModernFlatGUIPack/Widgets/WBP_LevelCompleteScreen.SetScore` (`/Game/ModernFlatGUIPack/DemoGame/Blueprints/BP_ScreenManager.LevelCompleteScreen` (`/Game/ModernFlatGUIPack/DemoGame/Blueprints/BPFL_Demo.GetScreenManager`)) (* (`self.CurrentLevel`) 2000)))

(fn `UserConstructionScript`)