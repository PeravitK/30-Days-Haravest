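; BP_Tree is a planted farm tree that affects humidity, pollution and temperature and can be uprooted.
; InitializeTree sets mesh and effects from TreeAttr or shows a dead mesh; living trees spawn a BP_TreeCountdown, starting its effects unless loaded from save.
; Overlaps update BP_Char's interaction target and outline and refresh stage icons across trees, plots and crops.
; In CuttingStage, interaction plays an input-locked montage, resets the plot, signals the countdown and destroys the tree.
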(event `self.ReceiveBeginPlay`
  ;[1 1 1] remove
)

(event `self.collision.OnComponentBeginOverlap`
  (params (OverlappedComponent :type "PrimitiveComponent Object Reference") (OtherActor :type "Actor Object Reference") (OtherComp :type "PrimitiveComponent Object Reference") (OtherBodyIndex :type Integer) (bFromSweep :type Boolean) (SweepResult :type "HitResult Structure (by ref)"))
  ;[1 1 1] add beginoverlap actor to currentoverlap&overlaparray
  (bind _asbp_char (cast `/Game/30DH/Character/BP_Char` OtherActor))
  (set `/Game/30DH/Character/BP_Char.CurrentOverlapObj` self _asbp_char)
  (`KismetArrayLibrary.Array_AddUnique` (`/Game/30DH/Character/BP_Char.OverlapObjArray` _asbp_char) self)
  (`self.Display Stage`)
  (`/Game/30DH/Character/BP_Char.DisplayObjOutline` _asbp_char))

(event `self.collision.OnComponentEndOverlap`
  (params (OverlappedComponent :type "PrimitiveComponent Object Reference") (OtherActor :type "Actor Object Reference") (OtherComp :type "PrimitiveComponent Object Reference") (OtherBodyIndex :type Integer))
  (bind _asbp_char (cast `/Game/30DH/Character/BP_Char` OtherActor))
  (bind _overlapobjarray (`/Game/30DH/Character/BP_Char.OverlapObjArray` _asbp_char))
  (`KismetArrayLibrary.Array_Remove` _overlapobjarray (`KismetArrayLibrary.Array_Find` _overlapobjarray self))
  ;[1 1 1] Check Currentoverlap == endoverlaptrigger?
  (if (== (`/Game/30DH/Character/BP_Char.CurrentOverlapObj` _asbp_char) self)
    ;[1 1 1] Check still have overlap in overlaparray?
    (if (`KismetArrayLibrary.Array_IsEmpty` _overlapobjarray)
      ;[1 1 1] if array empty -> currentoverlap = empty too
      (set `/Game/30DH/Character/BP_Char.CurrentOverlapObj` null _asbp_char)
      (else
        ;[1 1 1] if array not empty -> set currentoverlap = last obj in array
        (set `/Game/30DH/Character/BP_Char.CurrentOverlapObj` (`|GetArrayItem` _overlapobjarray (`KismetArrayLibrary.Array_LastIndex` _overlapobjarray)) _asbp_char)))
    (`/Game/30DH/Character/BP_Char.DisplayObjOutline` _asbp_char)
    (`self.Display Stage`)))

(event `self.ReceiveTick`
  (params (DeltaSeconds :type "Float (single-precision)")))

(event `InteractTree`
  (if (`self.CuttingStage`)
    (`self.InteractAction`)
    (`KismetSystemLibrary.Delay` 2.3)
    (`self.Remove Tree`)
    (`GameplayStatics.PlaySound2D` "/Game/Interface_And_Item_Sounds/WAV/Pop_04.Pop_04" 1.0 1.0 0.0 null null)))

(event `InteractAction`
  (bind _returnvalue (`GameplayStatics.GetPlayerController` 0))
  ;[1 1 1] disableinput -> playmontage -> delay -> enableinput
  (bind _returnvalue_2 (`GameplayStatics.GetActorOfClass` "/Game/30DH/Character/BP_Char.BP_Char_C"))
  (`self.DisableInput` _returnvalue_2 _returnvalue)
  (bind _mesh (`Character.Mesh` _returnvalue_2))
  (`|PlayMontage` _mesh "/Game/30DH/Character/Anim/Animation_farm.Animation_farm"
    (:`then`
      (`KismetSystemLibrary.Delay` 2.3)
      (`AnimInstance.Montage_Stop` (`SkeletalMeshComponent.GetAnimInstance` _mesh) 0.2 "/Game/30DH/Character/Anim/Animation_farm.Animation_farm")
      (`self.EnableInput` _returnvalue_2 _returnvalue))))

(fn `++`
  (params (NewParam :type Integer))
  (if (< NewParam 0)
    _))

(fn `Display Stage`
  (`|ExecutionSequence`
    (:`then_0`
      (if (`self.CuttingStage`)
        (bind _outactors (`GameplayStatics.GetAllActorsOfClass` "BP_Tree_C"))
        (for _array_element _outactors
          (bind _stageicon (`/Game/30DH/Farm/BP_Tree.StageIcon` _array_element))
          (`SceneComponent.SetVisibility` _stageicon false false)
          (set `BillboardComponent.Sprite` "/Game/30DH/Farm/StageIcon/uproot.uproot" _stageicon)
          (`SceneComponent.SetVisibility` _stageicon true false))
        (else
          (bind _outactors_2 (`GameplayStatics.GetAllActorsOfClass` "BP_Tree_C"))
          (for _array_element_2 _outactors_2
            (if (`/Game/30DH/Farm/BP_Tree.IsDead` _array_element_2)
              (bind _stageicon_2 (`/Game/30DH/Farm/BP_Tree.StageIcon` _array_element_2))
              (`BillboardComponent.SetSprite` _stageicon_2 "/Game/30DH/Farm/StageIcon/dead.dead")
              (`SceneComponent.SetVisibility` _stageicon_2 true false)
              (else
                (`BillboardComponent.SetSprite` _stageicon_2 null)
                (`SceneComponent.SetVisibility` _stageicon_2 false false)))))))
    (:`then_1`
      (bind _outactors_3 (`GameplayStatics.GetAllActorsOfClass` "/Game/30DH/Farm/BP_Plot.BP_Plot_C"))
      (`/Game/30DH/Farm/BP_Plot.DisplayStage` _outactors_3))
    (:`then_2`
      (bind _outactors_4 (`GameplayStatics.GetAllActorsOfClass` "/Game/30DH/Farm/BP_Crop.BP_Crop_C"))
      (`/Game/30DH/Farm/BP_Crop.DisplayStage` _outactors_4))))

(fn `HumidityValue`)

(fn `InitializeTree`
  (params (TreeID :type Integer))
  (bind _outline (`self.Outline`))
  (bind _outline_2 (`self.Outline`))
  (bind (_icon _mesh _humidity _pollution _temperature) (break `/Game/30DH/Farm/Tree` (`|GetArrayItem` (`self.TreeAttr`) (`self.TreeID`))))
  (`|ExecutionSequence`
    (:`then_0`
      (set `self.TreeID` (- TreeID 6)))
    (:`then_1`
      (if (`self.IsDead`)
        (`StaticMeshComponent.SetStaticMesh` (`self.Tree`) "/Game/PolygonFarm/Meshes/Environments/DeadTree.DeadTree")
        (`StaticMeshComponent.SetStaticMesh` _outline_2 "/Game/PolygonFarm/Meshes/Environments/DeadTree.DeadTree")
        (`PrimitiveComponent.SetMaterial` _outline_2 0 "/Game/30DH/Character/M_Outline_Inst.M_Outline_Inst")
        (`SceneComponent.SetVisibility` (`self.Tree`) true false)
        (else
          (`StaticMeshComponent.SetStaticMesh` (`self.Tree`) _mesh)
          (`StaticMeshComponent.SetStaticMesh` _outline _mesh)
          (`PrimitiveComponent.SetMaterial` _outline 0 "/Game/30DH/Character/M_Outline_Inst.M_Outline_Inst")
          (`SceneComponent.SetVisibility` (`self.Tree`) true false))))
    (:`then_2`
      (set `self.HumidityEffect` _humidity)
      (`self.HumidityValue`))
    (:`then_3`
      (set `self.PollutionEffect` _pollution)
      (`self.PollutionValue`))
    (:`then_4`
      (set `self.TemperatureEffect` _temperature)
      (`self.TemperatureValue`))
    (:`then_5`
      ;[1 1 1] Spawn env adapter
      (if (not (`self.IsDead`))
        (bind _returnvalue (`|SpawnActorFromClass` "/Game/30DH/Environment/BP_TreeCountdown.BP_TreeCountdown_C" (`KismetMathLibrary.MakeTransform` (`KismetMathLibrary.MakeVector` (.x (`SceneComponent.K2_GetComponentLocation` (`self.Tree`))) (.y (`SceneComponent.K2_GetComponentLocation` (`self.Tree`))) (+ (.z (`SceneComponent.K2_GetComponentLocation` (`self.Tree`))) 30.0))) "Undefined" "MultiplyWithRoot" null null))
        (set `self.TreeCountdown` _returnvalue)
        (if (not (`self.SpawnFromLoad`))
          (`/Game/30DH/Environment/BP_TreeCountdown.PollutionStart` _returnvalue (`self.PollutionEffect`))
          (`/Game/30DH/Environment/BP_TreeCountdown.TempStart` _returnvalue (`self.TemperatureEffect`))
          (`/Game/30DH/Environment/BP_TreeCountdown.HumidityStart` _returnvalue (`self.HumidityEffect`)))))))

(fn `PollutionValue`)

(fn `Remove Tree`
  (bind _treecountdown (`self.TreeCountdown`))
  (bind _asbp_plot (cast `/Game/30DH/Farm/BP_Plot` (`self.PlantedTileTree`)))
  (`/Game/30DH/Farm/BP_Plot.ResetFromTree` _asbp_plot)
  (`/Engine/EditorBlueprintResources/StandardMacros.IsValid` (`self.TreeCountdown`)
    (:`Is Valid`
      (set `/Game/30DH/Environment/BP_TreeCountdown.IsReset` true _treecountdown)
      (set `/Game/30DH/Environment/BP_TreeCountdown.TempCutting` true _treecountdown)
      (set `/Game/30DH/Environment/BP_TreeCountdown.HumidityCutting` true _treecountdown)
      (set `/Game/30DH/Environment/BP_TreeCountdown.PollutionCutting` true _treecountdown)
      (`/Game/30DH/Environment/BP_TreeCountdown.PollutionStart` _treecountdown (`self.PollutionEffect`))
      (`/Game/30DH/Environment/BP_TreeCountdown.TempStart` _treecountdown (`self.TemperatureEffect`))
      (`/Game/30DH/Environment/BP_TreeCountdown.HumidityStart` _treecountdown (`self.HumidityEffect`))
      (`self.K2_DestroyActor`))
    (:`Is Not Valid`
      (`self.K2_DestroyActor`))))

(fn `TemperatureValue`)

(fn `UserConstructionScript`)