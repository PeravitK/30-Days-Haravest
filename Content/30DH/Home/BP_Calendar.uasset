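; BP_Calendar is a calendar object in the home level that the player can open to view a calendar check widget.
; Its collision registers it in BP_Char's overlap array and current-overlap slot, refreshing the outline and falling back to the last overlapped object on exit.
; DisplayCalendar and CloseCalendar add or remove the WB_Calendar_check widget with a click sound, disabling and restoring the character's movement.
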(event `self.collision.OnComponentBeginOverlap`
  (params (OverlappedComponent :type "PrimitiveComponent Object Reference") (OtherActor :type "Actor Object Reference") (OtherComp :type "PrimitiveComponent Object Reference") (OtherBodyIndex :type Integer) (bFromSweep :type Boolean) (SweepResult :type "HitResult Structure (by ref)"))
  ;[1 1 1] add beginoverlap actor to currentoverlap&overlaparray
  (bind _asbp_char (cast `/Game/30DH/Character/BP_Char` OtherActor))
  (set `/Game/30DH/Character/BP_Char.CurrentOverlapObj` self _asbp_char)
  (`KismetArrayLibrary.Array_AddUnique` (`/Game/30DH/Character/BP_Char.OverlapObjArray` _asbp_char) self)
  (`/Game/30DH/Character/BP_Char.DisplayObjOutline` _asbp_char))

(event `self.collision.OnComponentEndOverlap`
  (params (OverlappedComponent :type "PrimitiveComponent Object Reference") (OtherActor :type "Actor Object Reference") (OtherComp :type "PrimitiveComponent Object Reference") (OtherBodyIndex :type Integer))
  (bind _asbp_char (cast `/Game/30DH/Character/BP_Char` OtherActor))
  (bind _overlapobjarray (`/Game/30DH/Character/BP_Char.OverlapObjArray` _asbp_char))
  (`KismetArrayLibrary.Array_Remove` _overlapobjarray (`KismetArrayLibrary.Array_Find` _overlapobjarray self))
  (if (== (`/Game/30DH/Character/BP_Char.CurrentOverlapObj` _asbp_char) self)
    ;[1 1 1] Check still have overlap in overlaparray?
    (if (`KismetArrayLibrary.Array_IsEmpty` _overlapobjarray)
      ;[1 1 1] if array empty -> currentoverlap = empty too
      (set `/Game/30DH/Character/BP_Char.CurrentOverlapObj` null _asbp_char)
      (else
        ;[1 1 1] if array not empty -> set currentoverlap = last obj in array
        (set `/Game/30DH/Character/BP_Char.CurrentOverlapObj` (`|GetArrayItem` _overlapobjarray (`KismetArrayLibrary.Array_LastIndex` _overlapobjarray)) _asbp_char)))
    (`/Game/30DH/Character/BP_Char.DisplayObjOutline` _asbp_char)))

(fn `CloseCalendar`
  (`/Engine/EditorBlueprintResources/StandardMacros.IsValid` (`self.WB_calendar_check`)
    (:`Is Valid`
      (`GameplayStatics.PlaySound2D` "/Game/Interface_And_Item_Sounds/WAV/Click_08.Click_08" 1.0 1.0 0.0 null null)
      (`Widget.RemoveFromParent` (`self.WB_calendar_check`))
      (bind _returnvalue (`GameplayStatics.GetActorOfClass` "/Game/30DH/Character/BP_Char.BP_Char_C"))
      (`CharacterMovementComponent.SetMovementMode` (`Character.CharacterMovement` _returnvalue) "MOVE_Walking" 0)
      (set `self.WB_calendar_check` null))))

(fn `DisplayCalendar`
  (`/Engine/EditorBlueprintResources/StandardMacros.IsValid` (`self.WB_calendar_check`)
    (:`Is Not Valid`
      (`GameplayStatics.PlaySound2D` "/Game/Interface_And_Item_Sounds/WAV/Click_08.Click_08" 1.0 1.0 0.0 null null)
      (bind _returnvalue (`|CreateWidget` "/Game/30DH/Home/Widget/WB_Calendar_check.WB_Calendar_check_C" (`GameplayStatics.GetPlayerController` 0)))
      (bind _output_get (set `self.WB_calendar_check` _returnvalue))
      (`UserWidget.AddToViewport` _output_get 10)
      (bind _returnvalue_2 (`GameplayStatics.GetActorOfClass` "/Game/30DH/Character/BP_Char.BP_Char_C"))
      (`CharacterMovementComponent.DisableMovement` (`Character.CharacterMovement` _returnvalue_2)))))

(fn `UserConstructionScript`)