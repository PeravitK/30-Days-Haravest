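; BP_Thrower is a demo-game actor that throws eggs toward the point clicked with the mouse.
; On left click it traces under the cursor against WorldStatic objects and, on a blocking hit, spawns a BP_Egg at its camera's location.
; It then applies a fixed-strength impulse to the egg's Ball component along the normalized direction from camera to hit point.
; A debug sphere draw at the hit location is left disconnected.
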(event `Key|LeftMouseButton`
  (params (Key :type "Key Structure"))
  (:`Pressed`
    (`|ExecutionSequence`
      (:`then_0`
        (set `self.MouseHit` (`PlayerController.GetHitResultUnderCursorForObjects` (`GameplayStatics.GetPlayerController` 0) (`|MakeArray` "ObjectTypeQuery1" :!type "EObjectTypeQuery Enum") false)))
      (:`then_1`
        (if (`GameplayStatics.BreakHitResult` (`self.MouseHit`))
          (`|ExecutionSequence`
            (:`then_1`
              (bind _returnvalue (`|SpawnActorFromClass` "/Game/ModernFlatGUIPack/DemoGame/Actors/BP_Egg.BP_Egg_C" (`KismetMathLibrary.MakeTransform` (`SceneComponent.K2_GetComponentLocation` (`self.Camera`))) "Undefined" "OverrideRootScale" null null))
              (`PrimitiveComponent.AddImpulse` (`/Game/ModernFlatGUIPack/DemoGame/Actors/BP_Egg.Ball` _returnvalue) (* (`KismetMathLibrary.Normal` (- (`.Location` (`GameplayStatics.BreakHitResult` (`self.MouseHit`))) (`SceneComponent.K2_GetComponentLocation` (`self.Camera`)))) 1000.0) "None" false))))))))

(fn `UserConstructionScript`)